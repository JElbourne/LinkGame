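; Game state for the Link game that restores overworld items and tracks a cycling kill count.
; On BeginPlay in L_Main, it reads the OverworldItems map from BP_LinkGameInstance and spawns each stored actor class at the location used as its key.
; IncrementKillCounter bumps and returns KillCounter, wrapping back to 1 once it passes 10.
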(event `self.ReceiveBeginPlay`
  (bind _asbp_link_game_instance (cast `/Game/_LinkGame/Blueprints/BP_LinkGameInstance` (`GameplayStatics.GetGameInstance`)))
  (set `self.As BP Link Game Instance` _asbp_link_game_instance)
  (bind _returnvalue (`GameplayStatics.GetCurrentLevelName` true))
  (if (`KismetStringLibrary.EqualEqual_StrStr` _returnvalue "L_Main")
    (`self.SpawnOverworldItems`)))

(event `SpawnOverworldItems`
  (bind _overworlditems (`/Game/_LinkGame/Blueprints/BP_LinkGameInstance.OverworldItems` (`self.As BP Link Game Instance`)))
  (bind _keys (`BlueprintMapLibrary.Map_Keys` _overworlditems))
  (for _array_element _keys
    (bind (_value _returnvalue) (`BlueprintMapLibrary.Map_Find` _overworlditems _array_element))
    (if _returnvalue
      (`|SpawnActorFromClass` _value (`KismetMathLibrary.MakeTransform` _array_element) "Undefined" "OverrideRootScale" null null))))

(fn `IncrementKillCounter`
  (returns (KillCounter :type Integer))
  (bind _result (`/Engine/EditorBlueprintResources/StandardMacros.IncrementInt` (`self.KillCounter`))
    (:`  `
      (if (> _result 10)
        (set `self.KillCounter` 1))
      (return (`self.KillCounter`)))))

(fn `UserConstructionScript`)