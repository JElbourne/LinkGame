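; BP_Link_GameInstance is the game instance that holds the player data and active save slot for the Link game.
; LoadGameData copies player data from a supplied save object and records its slot name.
; SaveGameData writes that data into a new BP_Link_SaveGame object and saves it to the current slot if one is set, printing a confirmation on success.
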(event `LoadGameData`
  (params (SaveGameData :type "/Game/_LinkGame/Blueprints/BP_Link_SaveGame Object Reference") (SaveSlot :type String))
  (set `self.PlayerData` (`/Game/_LinkGame/Blueprints/BP_Link_SaveGame.PlayerData` SaveGameData))
  (set `self.CurrentSaveSlot` SaveSlot))

(event `SaveGameData`
  (if (not (`KismetStringLibrary.IsEmpty` (`self.CurrentSaveSlot`)))
    (bind _returnvalue (`GameplayStatics.CreateSaveGameObject` "/Game/_LinkGame/Blueprints/BP_Link_SaveGame.BP_Link_SaveGame_C"))
    (set `/Game/_LinkGame/Blueprints/BP_Link_SaveGame.PlayerData` (`self.PlayerData`) _returnvalue)
    (bind _returnvalue_2 (`GameplayStatics.SaveGameToSlot` _returnvalue (`self.CurrentSaveSlot`)))
    (if _returnvalue_2
      (`KismetSystemLibrary.PrintString` "SAVED"))))