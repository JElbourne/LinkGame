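; BP_Tektite is a jumping enemy that hops to random points clamped around its zone coordinates, pausing randomly between jumps.
; A timeline drives each arc by lerping position and height, and overlapping a non-player while falling stops it and records the landing height.
; Overlapping the player's capsule applies damage.
; Death notifies BP_LinkGameState and spawns an item chosen by the incremented kill counter.
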(event `self.ReceiveBeginPlay`
  (`self.PickNextLocation`)
  (set `self.Health` 1.0))

(event `DestroyEnemy`
  (`self.K2_DestroyActor`))

(event `PickNextLocation`
  (bind (_returnvalue_x _returnvalue_y) (`KismetMathLibrary.BreakVector` (`self.K2_GetActorLocation`)))
  (bind (_zonecoords_x _zonecoords_y) (`KismetMathLibrary.BreakVector2D` (`self.ZoneCoords`)))
  (set `self.NextLocation` (`KismetMathLibrary.MakeVector` (`KismetMathLibrary.FClamp` (+ _returnvalue_x (`KismetMathLibrary.RandomFloatInRange` -300.0 300.0)) (- _zonecoords_x 500.0) (+ _zonecoords_x 500.0)) (`KismetMathLibrary.FClamp` (+ _returnvalue_y (`KismetMathLibrary.RandomFloatInRange` -500.0 500.0)) (- _zonecoords_y 700.0) (+ _zonecoords_y 700.0)) 0.0))
  (`self.JumpToLocation`))

(event `JumpToLocation`
  (bind _output_get (set `self.CurrentLocation` (`self.K2_GetActorLocation`)))
  (if (> (`KismetMathLibrary.Vector_Distance` _output_get (`self.NextLocation`)) 250.0)
    (`self.Timeline_JumpTo`
      (:`then`
        (bind (_direction _travelpercentage _jumpheightpercentage) (`Timeline|Timeline_JumpTo` :!via `PlayFromStart` :!label _label)
          (:`Update`
            (bind (_returnvalue_x _returnvalue_y) (`KismetMathLibrary.BreakVector` (`KismetMathLibrary.VLerp` (`self.CurrentLocation`) (`self.NextLocation`) _travelpercentage)))
            (`self.K2_SetActorLocation` (`KismetMathLibrary.MakeVector` _returnvalue_x _returnvalue_y (`KismetMathLibrary.Lerp` (`self.LastHeight`) (`self.JumpHeight`) _jumpheightpercentage))))
          (:`Finished`
            (`self.StopMoving`))
          (:`Falling`
            (set `self.Falling` true)
            (set `self.LastHeight` 0.0))))
      (:`else`))
    (else
      (`self.StopMoving`))))

(event `StopMoving`
  (`|ExecutionSequence`
    (:`then_0`
      (goto _label :!via `Stop`))
    (:`then_1`
      (`KismetSystemLibrary.Delay` (`KismetMathLibrary.RandomFloatInRange` 1.0 5.0))
      (`self.PickNextLocation`)
      (set `self.Falling` false))))

(event `self.StaticMesh.OnComponentBeginOverlap`
  (params (OverlappedComponent :type "PrimitiveComponent Object Reference") (OtherActor :type "Actor Object Reference") (OtherComp :type "PrimitiveComponent Object Reference") (OtherBodyIndex :type Integer) (bFromSweep :type Boolean) (SweepResult :type "HitResult Structure (by ref)"))
  (bind (_returnvalue_x _returnvalue_y _returnvalue_z) (`KismetMathLibrary.BreakVector` (`self.K2_GetActorLocation`)))
  ;[1 1 1] Collision
  (bind _astemp_player (cast `/Game/_LinkGame/Characters/Player/TempPlayer` OtherActor)
    (:`then`
      (if (== OtherComp (`Character.CapsuleComponent` _astemp_player))
        (`GameplayStatics.ApplyDamage` _astemp_player (`self.AttackDamage`))))
    (:`CastFailed`
      (if (`self.Falling`)
        (`self.StopMoving`)
        (set `self.LastHeight` _returnvalue_z)))))

(event `self.Die`
  ;[1 1 1] On Death
  (bind _asbp_link_game_state (cast `/Game/_LinkGame/Blueprints/BP_LinkGameState` (`GameplayStatics.GetGameState`)))
  (bind _output_get (set `self.As BP Link Game State` _asbp_link_game_state))
  (`/Game/_LinkGame/Blueprints/BP_LinkGameState.EnemyDied` _output_get (`self.EnemyId`))
  (`self.DropItem`)
  (`self.K2_DestroyActor`))

(event `DropItem`
  ;[1 1 1] On Death
  (bind _killcounter (`/Game/_LinkGame/Blueprints/BP_LinkGameState.IncrementKillCounter` (`self.As BP Link Game State`)))
  (switch `int` (`KismetMathLibrary.RandomInteger` 3)
    (:`0`
      _)
    (:`1`
      _)
    (:`2`
      _))
  (bind (_value _returnvalue) (`BlueprintMapLibrary.Map_Find` (`self.ItemDropChoices`) _killcounter))
  (if _returnvalue
    (`|SpawnActorFromClass` _value (`KismetMathLibrary.MakeTransform` (`self.K2_GetActorLocation`)) "Undefined" "OverrideRootScale" null null false null)))

(fn `UserConstructionScript`)