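; Peahat enemy for a Zelda-style game that cycles between resting, taking off, wandering in random directions within its zone bounds, and landing.
; Timelines drive each step and the height change, landing after a random step count; non-player overlaps mid-transition interrupt it.
; Touching the player's capsule deals damage.
; Death notifies the game state and may drop a kill-counter-based item; the enemy also despawns when the camera finishes moving.
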(event `self.ReceiveBeginPlay`
  (bind _astemp_player (cast `/Game/_LinkGame/Characters/Player/TempPlayer` (`GameplayStatics.GetPlayerCharacter` 0)))
  (set `self.As Temp Player` _astemp_player)
  (add `LinkMainCamera.OnFinishedMoving` (`self.CameraReference`) (delegate `DestroyEnemy`))
  (`self.WaitToFly`))

(event `DestroyEnemy`
  (`self.K2_DestroyActor`))

(event `self.Die`
  ;[1 1 1] On Death
  (bind _asbp_link_game_state (cast `/Game/_LinkGame/Blueprints/BP_LinkGameState` (`GameplayStatics.GetGameState`)))
  (bind _output_get (set `self.As BP Link Game State` _asbp_link_game_state))
  (`GameplayStatics.PlaySound2D` "/Game/_LinkGame/Audio/SoundEffects/LOZ_Enemy_Die.LOZ_Enemy_Die" 1.0 1.0 0.0 null null)
  (`/Game/_LinkGame/Blueprints/BP_LinkGameState.EnemyDied` _output_get (`self.EnemyId`))
  (`self.DropItem`)
  (`self.K2_DestroyActor`))

(event `DropItem`
  ;[1 1 1] On Death
  (bind _killcounter (`/Game/_LinkGame/Blueprints/BP_LinkGameState.IncrementKillCounter` (`self.As BP Link Game State`)))
  (switch `int` (`KismetMathLibrary.RandomInteger` 3)
    (:`0`
      _)
    (:`1`
      _))
  (bind (_value _returnvalue) (`BlueprintMapLibrary.Map_Find` (`self.ItemDropChoices`) _killcounter))
  (if _returnvalue
    (`|SpawnActorFromClass` _value (`KismetMathLibrary.MakeTransform` (`self.K2_GetActorLocation`)) "Undefined" "OverrideRootScale" null 0 null false null)))

(event `MoveForward`
  ;[1 1 1] Move the Character
  (set `self.CurrentLocation` (`self.K2_GetActorLocation`))
  (`self.FindNextLocation`)
  (set `self.MaxDistance` (`KismetMathLibrary.RandomIntegerInRange` 15 25))
  (`self.Timeline_EnemyWalk` :!label _label
    (:`then`
      (bind (_direction _amountmoved) (`Timeline|Timeline_EnemyWalk` :!via `PlayFromStart` :!label _label_2)
        (:`Update`
          (bind _inbounds (`self.CheckWithinAreaBounds`))
          (if _inbounds
            (bind (_sweephitresult _returnvalue) (`self.K2_SetActorLocation` (`KismetMathLibrary.VLerp` (`self.CurrentLocation`) (`self.NextLocation`) _amountmoved)))
            (else
              (`self.StopMoving` false))))
        (:`Finished`
          (bind _result (`/Engine/EditorBlueprintResources/StandardMacros.IncrementInt` (`self.TotalDistance`))
            (:`  `
              (if (> _result (`self.MaxDistance`))
                (`self.FlyMovement` true)
                (else
                  (set `self.CurrentLocation` (`self.NextLocation`))
                  (`self.FindNextLocation`)
                  (goto _label))))))))
    (:`else`)))

(event `StopMoving`
  (params (`with delay` :type Boolean))
  ;[1 1 1] Move the Character
  (`|ExecutionSequence`
    (:`then_0`
      (goto _label_2 :!via `Stop`))
    (:`then_1`
      (bind _result (`/Engine/EditorBlueprintResources/StandardMacros.IncrementInt` (`self.TotalDistance`))
        (:`  `
          (if (> _result (`self.MaxDistance`))
            (`self.FlyMovement` true)
            (else
              (`self.FindNextLocation`)
              (goto _label))))))))

(event `FindNextLocation`
  ;[1 1 1] Move the Character
  (set `self.NextLocation` (+ (`KismetArrayLibrary.Array_Random` (`self.Directions`)) (`self.CurrentLocation`)))
  (bind _inbounds (`self.CheckWithinAreaBounds`))
  (if (not _inbounds)
    (`self.StopMoving` false)))

(event `WaitToFly`
  ;[1 1 1] Fly
  (`KismetSystemLibrary.Delay` (`KismetMathLibrary.RandomFloatInRange` 1.0 3.0))
  (set `self.TotalDistance` 0)
  (`self.FlyMovement` false))

(event `self.StaticMesh.OnComponentBeginOverlap`
  (params (OverlappedComponent :type "PrimitiveComponent Object Reference") (OtherActor :type "Actor Object Reference") (OtherComp :type "PrimitiveComponent Object Reference") (OtherBodyIndex :type Integer) (bFromSweep :type Boolean) (SweepResult :type "HitResult Structure (by ref)"))
  (bind (_returnvalue_x _returnvalue_y _returnvalue_z) (`KismetMathLibrary.BreakVector` (`self.K2_GetActorLocation`)))
  ;[1 1 1] Collision
  (bind _astemp_player (cast `/Game/_LinkGame/Characters/Player/TempPlayer` OtherActor)
    (:`then`
      (if (== OtherComp (`Character.CapsuleComponent` _astemp_player))
        (`GameplayStatics.ApplyDamage` _astemp_player (`self.Damage`))))
    (:`CastFailed`
      (if (`self.FlyingTransitioning`)
        (`self.StopLanding`)
        (set `self.LastHeight` _returnvalue_z)))))

(event `FlyMovement`
  (params (Landing :type Boolean))
  (bind (_returnvalue_x _returnvalue_y) (`KismetMathLibrary.BreakVector` (`self.K2_GetActorLocation`)))
  ;[1 1 1] Fly
  (set `self.FlyingTransitioning` true)
  (if (not Landing)
    (bind (_direction _takeoffpercentage) (`Timeline|Timeline_Burrow` :!via `PlayFromStart` :!label _label_3)
      (:`Update`
        (`self.K2_SetActorLocation` (`KismetMathLibrary.MakeVector` _returnvalue_x _returnvalue_y (`KismetMathLibrary.Lerp` (`self.LastHeight`) (`self.FlyingHeight`) _takeoffpercentage))))
      (:`Finished`
        (if Landing
          (`self.WaitToFly`)
          (else
            (`self.MoveForward`)))
        (set `self.FlyingTransitioning` false)))
    (else
      (set `self.LastHeight` 0.0)
      (goto _label_3 :!via `ReverseFromEnd`))))

(event `StopLanding`
  ;[1 1 1] Fly
  (`|ExecutionSequence`
    (:`then_0`
      (goto _label_3 :!via `Stop`))
    (:`then_1`
      (`self.WaitToFly`))))

(fn `CheckWithinAreaBounds`
  (returns (InBounds :type Boolean))
  (bind (_zonecoords_x _zonecoords_y) (`KismetMathLibrary.BreakVector2D` (`self.ZoneCoords`)))
  (bind (_nextlocation_x _nextlocation_y) (`KismetMathLibrary.BreakVector` (`self.NextLocation`)))
  (return (not (or (> (`KismetMathLibrary.Abs` (- (`KismetMathLibrary.Abs` _zonecoords_x) (`KismetMathLibrary.Abs` _nextlocation_x))) 500.0) (> (`KismetMathLibrary.Abs` (- (`KismetMathLibrary.Abs` _zonecoords_y) (`KismetMathLibrary.Abs` _nextlocation_y))) 700.0)))))

(fn `UserConstructionScript`)