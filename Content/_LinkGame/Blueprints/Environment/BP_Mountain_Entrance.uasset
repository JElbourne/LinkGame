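; Mountain cave entrance that moves the player between the overworld and a cave by opening a named level.
; On overlap it freezes the player, saves player data to the GameInstance and updates its cave record, keyed by Arrow world location, flagging the item condition if potions are activated.
; Overworld-bound trips load after a short delay; otherwise it stores camera location and cave ID, then plays a timeline-driven stair descent before loading.
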(event `self.ReceiveBeginPlay`
  (bind _asbp_link_game_instance (cast `/Game/_LinkGame/Blueprints/BP_Link_GameInstance` (`GameplayStatics.GetGameInstance`)))
  (set `self.As BP Link Game Instance` _asbp_link_game_instance)
  (bind _asbp_player_controller (cast `/Game/_LinkGame/Blueprints/Controllers/BP_PlayerController` (`GameplayStatics.GetPlayerController` 0)))
  (set `self.As BP Player Controller` _asbp_player_controller)
  (set `self.CaveID` (`SceneComponent.K2_GetComponentLocation` (`self.Arrow`)))
  (`self.UpdateCaveData`))

(event `UpdateCaveData`
  (bind (_value _returnvalue) (`BlueprintMapLibrary.Map_Find` (`/Game/_LinkGame/Blueprints/BP_Link_GameInstance.OverworldCaveData` (`self.As BP Link Game Instance`)) (`self.CaveID`)))
  (if _returnvalue
    (set `self.CaveData` _value)))

(event `self.Collider.OnComponentBeginOverlap`
  (params (OverlappedComponent :type "PrimitiveComponent Object Reference") (OtherActor :type "Actor Object Reference") (OtherComp :type "PrimitiveComponent Object Reference") (OtherBodyIndex :type Integer) (bFromSweep :type Boolean) (SweepResult :type "HitResult Structure (by ref)"))
  (bind _as_bp_link_game_instance (`self.As BP Link Game Instance`))
  (bind _as_bp_link_game_instance_2 (`self.As BP Link Game Instance`))
  (bind _overworldcavedata (`/Game/_LinkGame/Blueprints/BP_Link_GameInstance.OverworldCaveData` _as_bp_link_game_instance))
  (bind (_value _returnvalue) (`BlueprintMapLibrary.Map_Find` _overworldcavedata (`self.CaveID`)))
  (bind _astemp_player (cast `/Game/_LinkGame/Characters/Player/TempPlayer` OtherActor))
  (set `LinkGameCharacter.bIsMovementFrozen` true _astemp_player)
  (`MovementComponent.StopMovementImmediately` (`Character.CharacterMovement` _astemp_player))
  (bind _playerdata (`/Game/_LinkGame/Characters/Player/TempPlayer.PlayerData` _astemp_player))
  (set `/Game/_LinkGame/Blueprints/BP_Link_GameInstance.PlayerData` _playerdata _as_bp_link_game_instance)
  (if _returnvalue
    (bind _output_get (set `self.CaveData` _value))
    (if (`.bIsItemsConditionMet_15_9A1B7F6044F7B8537AAFDDB861026635` (break `/Game/_LinkGame/Structs/ST_CaveData` _output_get))
      _
      (elif (`.PotionsActivated_25_26E1CB4C4E5C1637C9A30ABCE2C7943C` (break `/Game/_LinkGame/Structs/ST_PlayerData` _playerdata))
        (bind _structout (setmembers `/Game/_LinkGame/Structs/ST_CaveData` :`StructRef` (`self.CaveData`) :`bIsItemsConditionMet` true))
        (`BlueprintMapLibrary.Map_Add` _overworldcavedata (`self.CaveID`) _structout)))
    (else
      (`BlueprintMapLibrary.Map_Add` _overworldcavedata (`self.CaveID`) (`self.CaveData`))))
  (bind _output_get_2 (set `/Game/_LinkGame/Blueprints/BP_Link_GameInstance.IsTravelingToOverworld` (`self.bIsTravelToOverworld`) (`self.As BP Link Game Instance`)))
  (if _output_get_2
    (`KismetSystemLibrary.Delay` 0.2)
    (`self.GoToCave`)
    (else
      (set `/Game/_LinkGame/Blueprints/BP_Link_GameInstance.OverworldCameraLocation` (`SceneComponent.K2_GetComponentLocation` (`/Game/_LinkGame/Blueprints/Cameras/BP_MainCamera.DefaultSceneRoot` (`/Game/_LinkGame/Blueprints/Controllers/BP_PlayerController.CurrentCamera` (`self.As BP Player Controller`)))) _as_bp_link_game_instance_2)
      (set `/Game/_LinkGame/Blueprints/BP_Link_GameInstance.OverworldCaveID` (`self.CaveID`) _as_bp_link_game_instance_2)
      (`self.PlayerEnterCaveAnim` _astemp_player))))

(event `PlayerEnterCaveAnim`
  (params (PlayerPawn :type "/Game/_LinkGame/Characters/Player/TempPlayer Object Reference"))
  (bind (_returnvalue_x _returnvalue_y) (`KismetMathLibrary.BreakVector` (`self.K2_GetActorLocation`)))
  (bind (_returnvalue_x_2 _returnvalue_y_2) (`KismetMathLibrary.BreakVector` (`self.K2_GetActorLocation` PlayerPawn)))
  (`GameplayStatics.PlaySound2D` "/Game/_LinkGame/Audio/SoundEffects/LOZ_Stairs.LOZ_Stairs" 1.0 1.0 0.0 null null)
  (`self.SetActorEnableCollision` PlayerPawn false)
  (`TimelineComponent.SetPlayRate` (`self.Timeline_EnterCave`) 1.0)
  (bind (_direction _steps) (`Timeline|Timeline_EnterCave` :!via `PlayFromStart`)
    (:`Update`
      (`self.K2_SetActorLocation` PlayerPawn (`KismetMathLibrary.MakeVector` (`KismetMathLibrary.Lerp` _returnvalue_x_2 (+ _returnvalue_x 20.0) _steps) (`KismetMathLibrary.Lerp` _returnvalue_y_2 _returnvalue_y _steps) (`KismetMathLibrary.Lerp` 50.0 20.0 _steps)) false false))
    (:`Finished`
      (`self.GoToCave`))))

(event `GoToCave`
  (`GameplayStatics.OpenLevel` (`self.Level Name`)))

(fn `UserConstructionScript`)