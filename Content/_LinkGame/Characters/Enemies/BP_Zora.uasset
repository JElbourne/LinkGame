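; BP_Zora is a Zelda-style Zora enemy that surfaces at random spots, fires at the player, then sinks and relocates.
; PickSpawnLocation retries random points around EnemyId until an object trace hits, then a reversible timeline raises the actor.
; It shoots BP_Fire_Projectile toward the player, lowers, hides and repeats.
; Death notifies the game state and may drop a kill-counter-based item; finished camera moves also destroy it.
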(event `self.ReceiveBeginPlay`
  (`self.SetActorHiddenInGame` true)
  (`SceneComponent.K2_AddRelativeLocation` (`self.StaticMesh`) (0.0 0.0 -120.0) false false)
  (add `LinkMainCamera.OnFinishedMoving` (`self.CameraReference`) (delegate `DestroyEnemy`))
  (`self.PickSpawn`))

(event `DestroyEnemy`
  (`self.K2_DestroyActor`))

(event `self.Die`
  ;[1 1 1] On Death
  (bind _asbp_link_game_state (cast `/Game/_LinkGame/Blueprints/BP_LinkGameState` (`GameplayStatics.GetGameState`)))
  (bind _output_get (set `self.As BP Link Game State` _asbp_link_game_state))
  (`GameplayStatics.PlaySound2D` "/Game/_LinkGame/Audio/SoundEffects/LOZ_Enemy_Die.LOZ_Enemy_Die" 1.0 1.0 0.0 null null)
  (`/Game/_LinkGame/Blueprints/BP_LinkGameState.EnemyDied` _output_get (`self.EnemyId`))
  (`self.DropItem`)
  (`self.K2_DestroyActor`))

(event `DropItem`
  ;[1 1 1] On Death
  (bind _killcounter (`/Game/_LinkGame/Blueprints/BP_LinkGameState.IncrementKillCounter` (`self.As BP Link Game State`)))
  (switch `int` (`KismetMathLibrary.RandomInteger` 3)
    (:`0`
      _)
    (:`1`
      _))
  (bind (_value _returnvalue) (`BlueprintMapLibrary.Map_Find` (`self.ItemDropChoices`) _killcounter))
  (if _returnvalue
    (`|SpawnActorFromClass` _value (`KismetMathLibrary.MakeTransform` (`self.K2_GetActorLocation`)) "Undefined" "OverrideRootScale" null 0 null false null)))

(event `PickSpawn`
  ;[1 1 1] Burrow
  (`KismetSystemLibrary.Delay` (`KismetMathLibrary.RandomFloatInRange` 0.25 1.0))
  (`self.PickSpawnLocation`))

(event `BurrowMovement`
  (params (BurrowDown :type Boolean))
  (bind (_returnvalue_x _returnvalue_y) (`KismetMathLibrary.BreakVector` (`self.K2_GetActorLocation`)))
  ;[1 1 1] Burrow
  (if BurrowDown
    (bind (_direction _depthpercentage) (`Timeline|Timeline_Burrow` :!via `PlayFromStart` :!label _label)
      (:`Update`
        (`self.K2_SetActorLocation` (`KismetMathLibrary.MakeVector` _returnvalue_x _returnvalue_y (`KismetMathLibrary.Lerp` 0.0 -120.0 _depthpercentage))))
      (:`Finished`
        (if BurrowDown
          (`self.HideAndWait`)
          (else
            (`self.ShootProjectile`)))))
    (else
      (`self.SetActorHiddenInGame` false)
      (goto _label :!via `ReverseFromEnd`))))

(event `HideAndWait`
  ;[1 1 1] Burrow
  (`self.SetActorHiddenInGame` true)
  (`KismetSystemLibrary.Delay` 1.0)
  (`self.PickSpawn`))

(event `ShootProjectile`
  (bind _returnvalue (`self.K2_GetActorLocation`))
  (set `self.ShotTargetRotation` (`KismetMathLibrary.FindLookAtRotation` _returnvalue (`self.K2_GetActorLocation` (`GameplayStatics.GetPlayerPawn` 0))))
  (`KismetSystemLibrary.Delay` 0.4)
  (`|SpawnActorFromClass` "/Game/_LinkGame/Blueprints/Weapons/Projectile/BP_Fire_Projectile.BP_Fire_Projectile_C" (`KismetMathLibrary.MakeTransform` _returnvalue (`self.ShotTargetRotation`) (0.25 0.25 0.25)) "AlwaysSpawn" "OverrideRootScale" self (`self.ZoneCoords`) 2.0 null)
  (`self.BurrowMovement` true))

(fn `CheckWithinAreaBounds`
  (returns (InBounds :type Boolean))
  (bind (_zonecoords_x _zonecoords_y) (`KismetMathLibrary.BreakVector2D` (`self.ZoneCoords`)))
  (bind (_nextlocation_x _nextlocation_y) (`KismetMathLibrary.BreakVector` (`self.NextLocation`)))
  (return (not (or (> (`KismetMathLibrary.Abs` (- (`KismetMathLibrary.Abs` _zonecoords_x) (`KismetMathLibrary.Abs` _nextlocation_x))) 500.0) (> (`KismetMathLibrary.Abs` (- (`KismetMathLibrary.Abs` _zonecoords_y) (`KismetMathLibrary.Abs` _nextlocation_y))) 700.0)))))

(fn `PickSpawnLocation`
  (bind (_enemyid_x _enemyid_y) (`KismetMathLibrary.BreakVector` (`self.EnemyId`)))
  (bind _returnvalue (`KismetMathLibrary.MakeVector` (+ _enemyid_x (`KismetMathLibrary.RandomFloatInRange` -100.0 100.0)) (+ _enemyid_y (`KismetMathLibrary.RandomFloatInRange` -300.0 300.0)) -120.0))
  (set `self.TotalDistance` 0)
  (for _ (range 51)
    (bind _output_get (set `self.WorldSpawnLocation` _returnvalue))
    (bind (_outhit _returnvalue_2) (`KismetSystemLibrary.LineTraceSingleForObjects` _output_get (+ _returnvalue (0.0 0.0 100.0)) (`self.Object Types`)))
    (if _returnvalue_2
      (`KismetSystemLibrary.PrintString` "FOUDN LCOATION")
      (`|ExecutionSequence`
        (:`then_0`
          (break))
        (:`then_1`
          (`self.K2_SetActorLocation` (`self.WorldSpawnLocation`))
          (`self.BurrowMovement` false))))))

(fn `UserConstructionScript`)