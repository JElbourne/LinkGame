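; Game instance that holds the persistent player data and overworld item state and handles loading and saving it.
; LoadTheSaveGame casts the given save object to BP_Link_SaveGame, caches it with its slot name, and copies its data into the instance.
; SaveTheGame writes the current data back into that cached save and saves it to the slot, printing a failure message when no valid slot or save exists.
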(event `LoadTheSaveGame`
  (params (SaveGameData :type "SaveGame Object Reference") (SaveSlot :type String))
  (bind _asbp_link_save_game (cast `/Game/_LinkGame/Blueprints/BP_Link_SaveGame` SaveGameData))
  (bind _output_get (set `self.As BP Link Save Game` _asbp_link_save_game))
  (set `self.CurrentSaveSlot` SaveSlot)
  (set `self.PlayerData` (`/Game/_LinkGame/Blueprints/BP_Link_SaveGame.PlayerData` _output_get))
  (set `self.OverworldItems` (`/Game/_LinkGame/Blueprints/BP_Link_SaveGame.OverworldItems` _output_get)))

(event `SaveTheGame`
  (bind _as_bp_link_save_game (`self.As BP Link Save Game`))
  (if (and (not (`KismetStringLibrary.IsEmpty` (`self.CurrentSaveSlot`))) (`KismetSystemLibrary.IsValid` (`self.As BP Link Save Game`)))
    (set `/Game/_LinkGame/Blueprints/BP_Link_SaveGame.PlayerData` (`self.PlayerData`) _as_bp_link_save_game)
    (set `/Game/_LinkGame/Blueprints/BP_Link_SaveGame.OverworldItems` (`self.OverworldItems`) _as_bp_link_save_game)
    (`GameplayStatics.SaveGameToSlot` (`self.As BP Link Save Game`) (`self.CurrentSaveSlot`))
    (else
      (`KismetSystemLibrary.PrintString` "FAILED TO SAVE"))))