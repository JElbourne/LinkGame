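; Red Leever enemy for a Zelda-style game that surfaces near the player, wanders on a grid and burrows away to reappear.
; It spawns two tiles ahead of the player, facing them, falling back to random zone points if a line trace is blocked.
; Timelines drive burrowing and bounded tile steps, and player contact deals damage.
; Death notifies game state and may drop kill-counter-based items; finished camera moves destroy it.
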(event `self.ReceiveBeginPlay`
  (bind _astemp_player (cast `/Game/_LinkGame/Characters/Player/TempPlayer` (`GameplayStatics.GetPlayerCharacter` 0)))
  (set `self.As Temp Player` _astemp_player)
  (set `self.Health` 1.0)
  (`self.SetActorHiddenInGame` true)
  (`SceneComponent.K2_AddRelativeLocation` (`self.StaticMesh`) (0.0 0.0 -120.0) false false)
  (add `LinkMainCamera.OnFinishedMoving` (`self.CameraReference`) (delegate `DestroyEnemy`))
  (`self.PickSpawnLocation`))

(event `DestroyEnemy`
  (`self.K2_DestroyActor`))

(event `self.Die`
  ;[1 1 1] On Death
  (bind _asbp_link_game_state (cast `/Game/_LinkGame/Blueprints/BP_LinkGameState` (`GameplayStatics.GetGameState`)))
  (bind _output_get (set `self.As BP Link Game State` _asbp_link_game_state))
  (`GameplayStatics.PlaySound2D` "/Game/_LinkGame/Audio/SoundEffects/LOZ_Enemy_Die.LOZ_Enemy_Die" 1.0 1.0 0.0 null null)
  (`/Game/_LinkGame/Blueprints/BP_LinkGameState.EnemyDied` _output_get (`self.EnemyId`))
  (`self.DropItem`)
  (`self.K2_DestroyActor`))

(event `DropItem`
  ;[1 1 1] On Death
  (bind _killcounter (`/Game/_LinkGame/Blueprints/BP_LinkGameState.IncrementKillCounter` (`self.As BP Link Game State`)))
  (switch `int` (`KismetMathLibrary.RandomInteger` 3)
    (:`0`
      _)
    (:`1`
      _))
  (bind (_value _returnvalue) (`BlueprintMapLibrary.Map_Find` (`self.ItemDropChoices`) _killcounter))
  (if _returnvalue
    (`|SpawnActorFromClass` _value (`KismetMathLibrary.MakeTransform` (`self.K2_GetActorLocation`)) "Undefined" "OverrideRootScale" null 0 null false null)))

(event `PickDirection`
  (bind _facingdirection (`self.FacingDirection`))
  ;[1 1 1] Move the Character
  ;;[1 1 1] Pick Rotation
  (`KismetSystemLibrary.Delay` 0.2)
  (switch `int` (`KismetMathLibrary.RandomInteger` 4)
    (:`0`
      (if (`|EnumEquality` _facingdirection "NewEnumerator0")
        (`self.PickDirection` :!label _label)
        (else
          (set `self.CurrentRotation` (struct))
          (set `self.FacingDirection` "NewEnumerator0")
          (`self.K2_SetActorRotation` (`self.CurrentRotation`) :!label _label_2)
          (`self.MoveForward`))))
    (:`1`
      (if (`|EnumEquality` _facingdirection "NewEnumerator2")
        (goto _label)
        (else
          (set `self.CurrentRotation` (struct :`Yaw` 270.0))
          (set `self.FacingDirection` "NewEnumerator2")
          (goto _label_2))))
    (:`2`
      (if (`|EnumEquality` _facingdirection "NewEnumerator1")
        (goto _label)
        (else
          (set `self.CurrentRotation` (struct :`Yaw` 180.0))
          (set `self.FacingDirection` "NewEnumerator1")
          (goto _label_2))))
    (:`3`
      (if (`|EnumEquality` _facingdirection "NewEnumerator3")
        (goto _label)
        (else
          (set `self.CurrentRotation` (struct :`Yaw` 90.0))
          (set `self.FacingDirection` "NewEnumerator3")
          (goto _label_2))))))

(event `MoveForward`
  (bind (_returnvalue_x _returnvalue_y _returnvalue_z) (`KismetMathLibrary.BreakVector` (`self.K2_GetActorLocation`)))
  ;[1 1 1] Move the Character
  (set `self.CurrentLocation` (`self.K2_GetActorLocation`))
  (`self.FindNextLocation`)
  (set `self.RandomDistance` (+ (`KismetMathLibrary.RandomInteger` 4) 1))
  (`self.Timeline_EnemyWalk` :!label _label_3
    (:`then`
      (bind (_direction _amountmoved) (`Timeline|Timeline_EnemyWalk` :!via `PlayFromStart` :!label _label_4)
        (:`Update`
          (bind _inbounds (`self.CheckWithinAreaBounds`))
          (if _inbounds
            (bind (_sweephitresult _returnvalue) (`self.K2_SetActorLocation` (`KismetMathLibrary.VLerp` (`self.CurrentLocation`) (`self.NextLocation`) _amountmoved)))
            (if (not _returnvalue)
              (`self.StopMoving` false)
              (`self.K2_SetActorLocation` (`KismetMathLibrary.MakeVector` (* (`KismetMathLibrary.Round` (/ _returnvalue_x 100.0)) 100.0) (+ (* (`KismetMathLibrary.Round` (/ (- _returnvalue_y 50.0) 100.0)) 100.0) 50.0) _returnvalue_z)))
            (else
              (`self.StopMoving` false))))
        (:`Finished`
          (bind _result (`/Engine/EditorBlueprintResources/StandardMacros.IncrementInt` (`self.TotalDistance`))
            (:`  `
              (if (> _result (`KismetMathLibrary.RandomIntegerInRange` 5 10))
                (`self.BurrowMovement` true)
                (else
                  (bind _result_2 (`/Engine/EditorBlueprintResources/StandardMacros.DecrementInt` (`self.RandomDistance`))
                    (:`  `
                      (if (> _result_2 0)
                        (set `self.CurrentLocation` (`self.NextLocation`))
                        (`self.FindNextLocation`)
                        (goto _label_3)
                        (else
                          (`self.StopMoving` false))))))))))))
    (:`else`)))

(event `StopMoving`
  (params (`with delay` :type Boolean))
  ;[1 1 1] Move the Character
  (`|ExecutionSequence`
    (:`then_0`
      (goto _label_4 :!via `Stop`))
    (:`then_1`
      (`/Engine/EditorBlueprintResources/StandardMacros.IncrementInt` (`self.TotalDistance`)
        (:`  `
          (`self.PickDirection`))))))

(event `FindNextLocation`
  (bind _currentlocation (`self.CurrentLocation`))
  ;[1 1 1] Move the Character
  (switch `/Game/_LinkGame/Blueprints/Enums/E_FacingDirection` (`self.FacingDirection`)
    (:`NewEnumerator0`
      (set `self.NextLocation` (+ _currentlocation (* (100.0 0.0 0.0) 1))))
    (:`NewEnumerator1`
      (set `self.NextLocation` (+ _currentlocation (* (-100.0 0.0 0.0) 1))))
    (:`NewEnumerator2`
      (set `self.NextLocation` (+ _currentlocation (* (0.0 -100.0 0.0) 1))))
    (:`NewEnumerator3`
      (set `self.NextLocation` (+ _currentlocation (* (0.0 100.0 0.0) 1)))))
  (bind _inbounds (`self.CheckWithinAreaBounds`))
  (if (not _inbounds)
    (`self.StopMoving` false)))

(event `self.StaticMesh.OnComponentBeginOverlap`
  (params (OverlappedComponent :type "PrimitiveComponent Object Reference") (OtherActor :type "Actor Object Reference") (OtherComp :type "PrimitiveComponent Object Reference") (OtherBodyIndex :type Integer) (bFromSweep :type Boolean) (SweepResult :type "HitResult Structure (by ref)"))
  (bind (_returnvalue_x _returnvalue_y _returnvalue_z) (`KismetMathLibrary.BreakVector` (`self.K2_GetActorLocation`)))
  ;[1 1 1] Collision
  (bind _astemp_player (cast `/Game/_LinkGame/Characters/Player/TempPlayer` OtherActor)
    (:`then`
      (if (== OtherComp (`Character.CapsuleComponent` _astemp_player))
        (`GameplayStatics.ApplyDamage` _astemp_player (`self.Damage`))))
    (:`CastFailed`
      (`KismetSystemLibrary.Delay` 0.2)
      (`self.StopMoving` true)
      (`self.K2_SetActorLocation` (`KismetMathLibrary.MakeVector` (* (`KismetMathLibrary.Round` (/ _returnvalue_x 100.0)) 100.0) (+ (* (`KismetMathLibrary.Round` (/ (- _returnvalue_y 50.0) 100.0)) 100.0) 50.0) _returnvalue_z)))))

(event `BurrowMovement`
  (params (BurrowDown :type Boolean))
  (bind (_returnvalue_x _returnvalue_y) (`KismetMathLibrary.BreakVector` (`self.K2_GetActorLocation`)))
  ;[1 1 1] Burrow
  (set `self.Burrowing` true)
  (if BurrowDown
    (bind (_direction _depthpercentage) (`Timeline|Timeline_Burrow` :!via `PlayFromStart` :!label _label_5)
      (:`Update`
        (`self.K2_SetActorLocation` (`KismetMathLibrary.MakeVector` _returnvalue_x _returnvalue_y (`KismetMathLibrary.Lerp` 10.0 -120.0 _depthpercentage))))
      (:`Finished`
        (if BurrowDown
          (`self.HideAndWait`)
          (else
            (`self.MoveForward`)
            (set `self.Burrowing` false)))))
    (else
      (`self.SetActorHiddenInGame` false)
      (goto _label_5 :!via `ReverseFromEnd`))))

(event `HideAndWait`
  ;[1 1 1] Burrow
  (`self.SetActorHiddenInGame` true)
  (`self.PickSpawnLocation`))

(fn `CheckWithinAreaBounds`
  (returns (InBounds :type Boolean))
  (bind (_zonecoords_x _zonecoords_y) (`KismetMathLibrary.BreakVector2D` (`self.ZoneCoords`)))
  (bind (_nextlocation_x _nextlocation_y) (`KismetMathLibrary.BreakVector` (`self.NextLocation`)))
  (return (not (or (> (`KismetMathLibrary.Abs` (- (`KismetMathLibrary.Abs` _zonecoords_x) (`KismetMathLibrary.Abs` _nextlocation_x))) 500.0) (> (`KismetMathLibrary.Abs` (- (`KismetMathLibrary.Abs` _zonecoords_y) (`KismetMathLibrary.Abs` _nextlocation_y))) 700.0)))))

(fn `PickSpawnLocation`
  (bind (_zonecoords_x _zonecoords_y) (`KismetMathLibrary.BreakVector2D` (`self.ZoneCoords`)))
  (bind _as_temp_player (`self.As Temp Player`))
  (bind (_returnvalue_x _returnvalue_y _returnvalue_z) (`KismetMathLibrary.BreakVector` (`self.K2_GetActorLocation` _as_temp_player)))
  (bind (_returnvalue_roll _returnvalue_pitch _returnvalue_yaw) (`KismetMathLibrary.BreakRotator` (`self.K2_GetActorRotation` _as_temp_player)))
  (bind _returnvalue (`KismetMathLibrary.MakeVector` (+ _zonecoords_x (`KismetMathLibrary.RandomFloatInRange` -400.0 400.0)) (+ _zonecoords_y (`KismetMathLibrary.RandomFloatInRange` -600.0 600.0)) 20.0))
  (bind _returnvalue_2 (`KismetMathLibrary.MakeVector` (* (`KismetMathLibrary.Round` (/ _returnvalue_x 100.0)) 100.0) (+ (* (`KismetMathLibrary.Round` (/ (- _returnvalue_y 50.0) 100.0)) 100.0) 50.0) _returnvalue_z))
  (bind (_returnvalue_x_2 _returnvalue_y_2) (`KismetMathLibrary.BreakVector` (+ _returnvalue_2 (`self.RelativeSpawnLocation`))))
  (set `self.TotalDistance` 0)
  (`/Engine/EditorBlueprintResources/StandardMacros.IsValid` _as_temp_player
    (:`Is Valid`
      (switch `string` (`KismetStringLibrary.Conv_IntToString` (`KismetMathLibrary.Round` _returnvalue_yaw))
        (:`0`
          (set `self.RelativeSpawnLocation` (200.0 0.0 0.0))
          (set `self.CurrentRotation` (struct :`Yaw` 180.0))
          (set `self.FacingDirection` "NewEnumerator1"))
        (:`90`
          (set `self.RelativeSpawnLocation` (0.0 200.0 0.0))
          (set `self.CurrentRotation` (struct :`Yaw` 270.0))
          (set `self.FacingDirection` "NewEnumerator2"))
        (:`-90`
          (set `self.RelativeSpawnLocation` (0.0 -200.0 0.0))
          (set `self.CurrentRotation` (struct :`Yaw` 90.0))
          (set `self.FacingDirection` "NewEnumerator3"))
        (:`-180`
          (set `self.RelativeSpawnLocation` (-200.0 0.0 0.0))
          (set `self.CurrentRotation` (struct))
          (set `self.FacingDirection` "NewEnumerator0")))
      (bind _output_get (set `self.WorldSpawnLocation` (`KismetMathLibrary.MakeVector` _returnvalue_x_2 _returnvalue_y_2 -120.0)))
      (bind (_outhit _returnvalue_3) (`KismetSystemLibrary.LineTraceSingleForObjects` _returnvalue_2 (`KismetMathLibrary.MakeVector` (.x _output_get) (.y _output_get) 20.0) (`self.Object Types`)))
      (if (not _returnvalue_3)
        (`self.K2_SetActorLocationAndRotation` (`self.WorldSpawnLocation`) (`self.CurrentRotation`) :!label _label)
        (`self.BurrowMovement` false)
        (else
          (for _ (range 51)
            (bind _output_get_2 (set `self.WorldSpawnLocation` _returnvalue))
            (bind (_outhit_2 _returnvalue_4) (`KismetSystemLibrary.LineTraceSingleForObjects` _output_get_2 (+ _returnvalue (100.0 0.0 20.0)) (`self.Object Types`)))
            (if (not _returnvalue_4)
              (`|ExecutionSequence`
                (:`then_0`
                  (break))
                (:`then_1`
                  (goto _label))))))))))

(fn `UserConstructionScript`)