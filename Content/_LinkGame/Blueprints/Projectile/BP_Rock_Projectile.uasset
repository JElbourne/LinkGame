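; BP_Rock_Projectile is a rock projectile actor that damages the player on contact.
; When its static mesh begins overlapping a TempPlayer, it applies its Damage value and destroys itself.
; Every tick it also destroys itself once it strays too far from ZoneCoords on X or Y, with the bounds check comparing absolute coordinate values, ignoring sign.
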(event `self.ReceiveTick`
  (params (DeltaSeconds :type "Float (single-precision)"))
  (bind _outofbounds (`self.CheckIfOutAreaBounds`))
  (if _outofbounds
    (`self.K2_DestroyActor`)))

(event `self.StaticMesh.OnComponentBeginOverlap`
  (params (OverlappedComponent :type "PrimitiveComponent Object Reference") (OtherActor :type "Actor Object Reference") (OtherComp :type "PrimitiveComponent Object Reference") (OtherBodyIndex :type Integer) (bFromSweep :type Boolean) (SweepResult :type "HitResult Structure (by ref)"))
  (bind _astemp_player (cast `/Game/_LinkGame/Characters/Player/TempPlayer` OtherActor))
  (`GameplayStatics.ApplyDamage` _astemp_player (`self.Damage`))
  (`self.K2_DestroyActor`))

(fn `CheckIfOutAreaBounds`
  (returns (OutOfBounds :type Boolean))
  (bind (_returnvalue_x _returnvalue_y) (`KismetMathLibrary.BreakVector` (`self.K2_GetActorLocation`)))
  (bind (_zonecoords_x _zonecoords_y) (`KismetMathLibrary.BreakVector2D` (`self.ZoneCoords`)))
  (return (or (> (`KismetMathLibrary.Abs` (- (`KismetMathLibrary.Abs` _zonecoords_x) (`KismetMathLibrary.Abs` _returnvalue_x))) 500.0) (> (`KismetMathLibrary.Abs` (- (`KismetMathLibrary.Abs` _zonecoords_y) (`KismetMathLibrary.Abs` _returnvalue_y))) 700.0))))

(fn `UserConstructionScript`)