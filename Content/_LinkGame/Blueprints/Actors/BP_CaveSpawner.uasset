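; BP_CaveSpawner populates a cave at BeginPlay with an NPC, dialogue text and items with costs.
; It reads the CaveType data from BP_LinkGameInstance, so the cave's contents depend on what the game instance holds.
; It spawns the NPC at a fixed point and writes the dialogue to a TextRenderActor.
; If the items condition is met, it spawns each valid item in an evenly spaced row, passing in its cost label.
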(event `self.ReceiveBeginPlay`
  (`KismetSystemLibrary.PrintString` "Hello")
  (bind _asbp_link_game_instance (cast `/Game/_LinkGame/Blueprints/BP_LinkGameInstance` (`GameplayStatics.GetGameInstance`)))
  (bind _output_get (set `self.As BP Link Game Instance` _asbp_link_game_instance))
  (set `self.CaveType` (`/Game/_LinkGame/Blueprints/BP_LinkGameInstance.CaveType` _output_get))
  (`TextRenderComponent.K2_SetText` (`TextRenderActor.TextRender` (`self.TextRenderActor`)) (`|FormatText` ""))
  (`self.SpawnNPC`)
  (`self.ShowDialogueText`)
  (`self.SpawnItems`))

(event `SpawnNPC`
  (bind _cavetype_npc (break `/Game/_LinkGame/Structs/ST_CaveType` (`self.CaveType`)))
  (`|SpawnActorFromClass` _cavetype_npc (`KismetMathLibrary.MakeTransform` (100.0 0.0 0.0) (struct :`Yaw` 90.0)) "Undefined" "OverrideRootScale" null null))

(event `ShowDialogueText`
  (bind (_cavetype_npc _cavetype_dialogue) (break `/Game/_LinkGame/Structs/ST_CaveType` (`self.CaveType`)))
  (`TextRenderComponent.K2_SetText` (`TextRenderActor.TextRender` (`self.TextRenderActor`)) (`|FormatText` _cavetype_dialogue)))

(event `SpawnItems`
  (bind (_cavetype_npc _cavetype_dialogue _cavetype_items _cavetype_itemscondition _cavetype_bisitemsconditionmet) (break `/Game/_LinkGame/Structs/ST_CaveType` (`self.CaveType`)))
  (if _cavetype_bisitemsconditionmet
    (for (_array_element _array_index) _cavetype_items
      (bind (_blueprint _costlabel) (break `/Game/_LinkGame/Structs/ST_Item` _array_element))
      (if (`KismetSystemLibrary.IsValidClass` _blueprint)
        (`|SpawnActorFromClass` _blueprint (`KismetMathLibrary.MakeTransform` (`KismetMathLibrary.MakeVector` -100.0 (- (* _array_index 200.0) 200.0) 25.0)) "Undefined" "OverrideRootScale" null _costlabel null)))))

(fn `UserConstructionScript`)