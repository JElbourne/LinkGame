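; Zone enemy spawner that spawns its enemies when the player's camera stops at its location.
; It polls the player controller on a timer until a camera exists, then checks position each time the camera finishes moving.
; A working copy of DefaultEnemies, keyed by spawn location as enemy ID, loses entries as the game state reports deaths.
; The copy resets once the camera stops at least the game mode's RespawnDistance away.
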(event `self.ReceiveBeginPlay`
  (`self.CopyDefaultEnemies`)
  (bind _asbp_player_controller (cast `/Game/_LinkGame/Blueprints/Controllers/Player/BP_PlayerController` (`GameplayStatics.GetPlayerController` 0)))
  (set `self.As BP Player Controller` _asbp_player_controller)
  (bind _returnvalue (`KismetSystemLibrary.K2_SetTimerDelegate` (delegate `RegisterCamera`) 0.1 true))
  (set `self.RegisterCameraTimer` _returnvalue)
  (bind _asbp_link_game_mode (cast `/Game/_LinkGame/Blueprints/BP_Link_GameMode` (`GameplayStatics.GetGameMode`)))
  (set `self.As BP Link Game Mode` _asbp_link_game_mode)
  (bind _asbp_link_game_state (cast `/Game/_LinkGame/Blueprints/BP_LinkGameState` (`GameplayStatics.GetGameState`)))
  (add `/Game/_LinkGame/Blueprints/BP_LinkGameState.EnemyDied` _asbp_link_game_state (delegate `EnemyHasDied`)))

(event `EnemyHasDied`
  (params (EnemyID :type "Vector Structure"))
  (`BlueprintMapLibrary.Map_Remove` (`self.RespawnEnemies`) EnemyID))

(event `RegisterCamera`
  (bind _currentcamera (`/Game/_LinkGame/Blueprints/Controllers/Player/BP_PlayerController.CurrentCamera` (`self.As BP Player Controller`)))
  (`/Engine/EditorBlueprintResources/StandardMacros.IsValid` _currentcamera
    (:`Is Valid`
      (set `self.Current Camera` _currentcamera)
      (`KismetSystemLibrary.K2_ClearAndInvalidateTimerHandle` (`self.RegisterCameraTimer`))
      (add `LinkMainCamera.OnFinishedMoving` (`self.Current Camera`) (delegate `CheckRespawn`))
      (if (== (`self.K2_GetActorLocation`) (`self.K2_GetActorLocation` (`self.Current Camera`)) :`ErrorTolerance` 100.0)
        (`self.SpawnEnemies`)))))

(event `CheckRespawn`
  (if (== (`SceneComponent.K2_GetComponentLocation` (`/Game/_LinkGame/Blueprints/Cameras/BP_MainCamera.DefaultSceneRoot` (`self.Current Camera`))) (`self.K2_GetActorLocation`) :`ErrorTolerance` 100.0)
    (`self.SpawnEnemies`)
    (elif (>= (`KismetMathLibrary.Vector_Distance` (`SceneComponent.K2_GetComponentLocation` (`/Game/_LinkGame/Blueprints/Cameras/BP_MainCamera.DefaultSceneRoot` (`self.Current Camera`))) (`self.K2_GetActorLocation`)) (`/Game/_LinkGame/Blueprints/BP_Link_GameMode.RespawnDistance` (`self.As BP Link Game Mode`)))
      (`self.CopyDefaultEnemies`))))

(event `SpawnEnemies`
  (bind (_returnvalue_x _returnvalue_y) (`KismetMathLibrary.BreakVector` (`self.K2_GetActorLocation`)))
  (bind _keys (`BlueprintMapLibrary.Map_Keys` (`self.RespawnEnemies`)))
  (for _array_element _keys
    (`|SpawnActorFromClass` (`BlueprintMapLibrary.Map_Find` (`self.RespawnEnemies`) _array_element) (`KismetMathLibrary.MakeTransform` _array_element (struct) (1.0 1.0 1.0)) "Undefined" "OverrideRootScale" null (`KismetMathLibrary.MakeVector2D` _returnvalue_x _returnvalue_y) _array_element (`self.Current Camera`) null)))

(event `CopyDefaultEnemies`
  (`BlueprintMapLibrary.Map_Clear` (`self.RespawnEnemies`))
  (bind _keys (`BlueprintMapLibrary.Map_Keys` (`self.DefaultEnemies`)))
  (for _array_element _keys
    (`BlueprintMapLibrary.Map_Add` (`self.RespawnEnemies`) _array_element (`BlueprintMapLibrary.Map_Find` (`self.DefaultEnemies`) _array_element)))
  (`KismetSystemLibrary.PrintString` (`KismetStringLibrary.Conv_IntToString` (`BlueprintMapLibrary.Map_Length` (`self.RespawnEnemies`)))))

(event `EnemyDestroyed`
  (params (EnemyID :type "Vector Structure"))
  (`BlueprintMapLibrary.Map_Remove` (`self.RespawnEnemies`) EnemyID))

(fn `UserConstructionScript`)