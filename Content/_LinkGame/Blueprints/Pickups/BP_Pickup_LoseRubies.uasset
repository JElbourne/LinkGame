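; BP_Pickup_LoseRubies is a pickup that makes the player lose rubies automatically.
; Shortly after BeginPlay it calls SpendRubies, then PickupAndDestroy, with no touch logic of its own.
; PickupAndDestroy hides the actor and notifies its spawner if valid, otherwise destroys itself.
; SetItemText blanks and hides the text render so no label shows.
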(event `self.ReceiveBeginPlay`
  (`parent.ReceiveBeginPlay`)
  (`KismetSystemLibrary.Delay` 0.5)
  (`self.SpendRubies` true)
  (`self.PickupAndDestroy`))

(event `self.PickupAndDestroy`
  (`self.SetActorHiddenInGame` true)
  (bind _spawnerreference (`self.SpawnerReference`)
    (:`then`
      (`/Game/_LinkGame/Blueprints/Actors/BP_CaveSpawner.ItemPickedUp` _spawnerreference (`self.As Temp Player`) self))
    (:`else`
      (`self.K2_DestroyActor`))))

(event `self.SetItemText`
  ;[1 1 1] Dont want to show text
  (`TextRenderComponent.K2_SetText` (`self.TextRender`) (`|FormatText` ""))
  (`SceneComponent.SetVisibility` (`self.TextRender`) false false))

(fn `UserConstructionScript`
  (`parent.UserConstructionScript`))