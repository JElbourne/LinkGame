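; Main gameplay camera that scrolls screen by screen across the map in a Zelda-style layout.
; On BeginPlay it restores the saved overworld position from the game instance when traveling there, then registers with the player controller.
; MoveCamera lerps it one fixed screen step in the given direction via a timeline, guarded against re-entry and flushing level streaming.
; When finished, it unfreezes player movement and signals completion.
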(event `self.ReceiveBeginPlay`
  (`self.SetOverworldLocation`)
  (bind _asbp_player_controller (cast `/Game/_LinkGame/Blueprints/Controllers/BP_PlayerController` (`GameplayStatics.GetPlayerController` 0)))
  (bind _output_get (set `self.As BP Player Controller` _asbp_player_controller))
  (`/Game/_LinkGame/Blueprints/Controllers/BP_PlayerController.RegisterMainCamera` _output_get self)
  (bind _astemp_player (cast `/Game/_LinkGame/Characters/Player/TempPlayer` (`GameplayStatics.GetPlayerCharacter` 0)))
  (set `self.As Temp Player` _astemp_player))

(event `MoveCamera`
  (params (MapDirection :type "Vector2D Structure"))
  (bind _returnvalue (`self.K2_GetActorLocation`))
  (bind (_returnvalue_x _returnvalue_y) (`KismetMathLibrary.BreakVector2D` (* MapDirection (1100.0 1600.0))))
  (`/Engine/EditorBlueprintResources/StandardMacros.DoOnce` false :!label _label
    (:`Completed`
      (set `self.OldLocation` _returnvalue)
      (set `self.NextLocation` (`KismetMathLibrary.MakeVector` (+ _returnvalue_x (.x _returnvalue)) (+ _returnvalue_y (.y _returnvalue)) (.z _returnvalue)))
      (bind (_direction _movepercentage) (`Timeline|CameraMoveTimepline` :!via `PlayFromStart`)
        (:`Update`
          (`GameplayStatics.FlushLevelStreaming`)
          (`self.K2_SetActorLocation` (`KismetMathLibrary.VLerp` (`self.OldLocation`) (`self.NextLocation`) _movepercentage)))
        (:`Finished`
          (`self.MovingFinished`)
          (goto _label :!via `Reset`))))))

(event `MovingFinished`
  (bind _astemp_player (cast `/Game/_LinkGame/Characters/Player/TempPlayer` (`GameplayStatics.GetPlayerCharacter` 0)))
  (set `LinkGameCharacter.bIsMovementFrozen` false _astemp_player)
  (`self.FinishedMovingCamera`))

(event `SetOverworldLocation`
  (bind _asbp_link_game_instance (cast `/Game/_LinkGame/Blueprints/BP_Link_GameInstance` (`GameplayStatics.GetGameInstance`)))
  (if (`/Game/_LinkGame/Blueprints/BP_Link_GameInstance.IsTravelingToOverworld` _asbp_link_game_instance)
    (`self.K2_SetActorLocation` (`/Game/_LinkGame/Blueprints/BP_Link_GameInstance.OverworldCameraLocation` _asbp_link_game_instance))))

(fn `UserConstructionScript`)