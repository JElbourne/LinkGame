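; BP_SwordProjectile is the hero's sword projectile, which damages Link enemies it overlaps.
; Each tick it checks whether it has strayed past fixed X/Y limits around its zone coordinates, comparing absolute coordinate values.
; On an enemy hit or leaving those bounds, it re-enables the hero's sword projectile availability and destroys itself, both only while the hero reference is valid.
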(event `self.ReceiveTick`
  (params (DeltaSeconds :type "Float (single-precision)"))
  (bind _heroreference (`self.HeroReference`))
  (bind _outofbounds (`self.CheckIfOutAreaBounds`))
  (if _outofbounds
    (`/Engine/EditorBlueprintResources/StandardMacros.IsValid` _heroreference
      (:`Is Valid`
        (set `/Game/_LinkGame/Characters/Player/TempPlayer.IsSwordProjectileAvailable` true _heroreference)
        (`self.K2_DestroyActor`)))))

(event `self.HitBox.OnComponentBeginOverlap`
  (params (OverlappedComponent :type "PrimitiveComponent Object Reference") (OtherActor :type "Actor Object Reference") (OtherComp :type "PrimitiveComponent Object Reference") (OtherBodyIndex :type Integer) (bFromSweep :type Boolean) (SweepResult :type "HitResult Structure (by ref)"))
  (bind _heroreference (`self.HeroReference`))
  (bind _aslink_enemy_base (cast `LinkEnemyBase` OtherActor))
  (`LinkEnemyBase.DamageEnemy` _aslink_enemy_base (`self.Damage`))
  (`/Engine/EditorBlueprintResources/StandardMacros.IsValid` _heroreference
    (:`Is Valid`
      (set `/Game/_LinkGame/Characters/Player/TempPlayer.IsSwordProjectileAvailable` true _heroreference)
      (`self.K2_DestroyActor`))))

(fn `CheckIfOutAreaBounds`
  (returns (OutOfBounds :type Boolean))
  (bind (_returnvalue_x _returnvalue_y) (`KismetMathLibrary.BreakVector` (`self.K2_GetActorLocation`)))
  (bind (_zonecoords_x _zonecoords_y) (`KismetMathLibrary.BreakVector2D` (`self.ZoneCoords`)))
  (return (or (> (`KismetMathLibrary.Abs` (- (`KismetMathLibrary.Abs` _zonecoords_x) (`KismetMathLibrary.Abs` _returnvalue_x))) 500.0) (> (`KismetMathLibrary.Abs` (- (`KismetMathLibrary.Abs` _zonecoords_y) (`KismetMathLibrary.Abs` _returnvalue_y))) 700.0))))

(fn `UserConstructionScript`)