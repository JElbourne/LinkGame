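; Octorok enemy that wanders a 100-unit grid in four directions and damages TempPlayer on mesh hit.
; It picks a new random facing, sometimes calls ShootProjectile (only a debug print), then walks a random number of tiles via a timeline lerp.
; Blocked sweeps snap it to the grid.
; Finishing, blockage or leaving the bounds around ZoneCoords stops it, and after a delay it picks again.
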(event `self.ReceiveBeginPlay`
  (`self.PickDirection`))

(event `PickDirection`
  (bind _facingdirection (`self.FacingDirection`))
  (switch `int` (`KismetMathLibrary.RandomInteger` 4)
    (:`0`
      ;[1 1 1] Pick Rotation
      (if (`|EnumEquality` _facingdirection "NewEnumerator0")
        (`self.PickDirection` :!label _label)
        (else
          (set `self.CurrentRotation` (struct))
          (set `self.FacingDirection` "NewEnumerator0")
          (`self.K2_SetActorRotation` (`self.CurrentRotation`) :!label _label_2)
          (switch `int` (`KismetMathLibrary.RandomInteger` 4)
            (:`0`
              (`self.MoveForward` :!label _label_3))
            (:`1`
              (goto _label_3))
            (:`2`
              (`self.ShootProjectile` :!label _label_4)
              (`self.MoveForward`))
            (:`3`
              (goto _label_4))))))
    (:`1`
      (if (`|EnumEquality` _facingdirection "NewEnumerator2")
        (goto _label)
        (else
          (set `self.CurrentRotation` (struct :`Yaw` 270.0))
          (set `self.FacingDirection` "NewEnumerator2")
          (goto _label_2))))
    (:`2`
      (if (`|EnumEquality` _facingdirection "NewEnumerator1")
        (goto _label)
        (else
          (set `self.CurrentRotation` (struct :`Yaw` 180.0))
          (set `self.FacingDirection` "NewEnumerator1")
          (goto _label_2))))
    (:`3`
      (if (`|EnumEquality` _facingdirection "NewEnumerator3")
        (goto _label)
        (else
          (set `self.CurrentRotation` (struct :`Yaw` 90.0))
          (set `self.FacingDirection` "NewEnumerator3")
          (goto _label_2))))))

(event `MoveForward`
  (bind (_returnvalue_x _returnvalue_y _returnvalue_z) (`KismetMathLibrary.BreakVector` (`self.K2_GetActorLocation`)))
  ;[1 1 1] Move the Character
  (set `self.CurrentLocation` (`self.K2_GetActorLocation`))
  (`self.FindNextLocation`)
  (set `self.RandomDistance` (+ (`KismetMathLibrary.RandomInteger` 5) 1))
  (bind (_direction _amountmoved) (`Timeline|Timeline_EnemyWalk` :!via `PlayFromStart` :!label _label_5)
    (:`Update`
      (bind _inbounds (`self.CheckWithinAreaBounds`))
      (if _inbounds
        (bind (_sweephitresult _returnvalue) (`self.K2_SetActorLocation` (`KismetMathLibrary.VLerp` (`self.CurrentLocation`) (`self.NextLocation`) _amountmoved) true))
        (if (not _returnvalue)
          (`self.StopMoving`)
          (`KismetSystemLibrary.PrintString` "SWEEP")
          (`self.K2_SetActorLocation` (`KismetMathLibrary.MakeVector` (* (`KismetMathLibrary.Round` (/ _returnvalue_x 100.0)) 100.0) (+ (* (`KismetMathLibrary.Round` (/ (- _returnvalue_y 50.0) 100.0)) 100.0) 50.0) _returnvalue_z)))
        (else
          (`self.StopMoving` :!label _label_6))))
    (:`Finished`
      (bind _result (`/Engine/EditorBlueprintResources/StandardMacros.DecrementInt` (`self.RandomDistance`))
        (:`  `
          (if (> _result 0)
            (set `self.CurrentLocation` (`self.NextLocation`))
            (`self.FindNextLocation`)
            (goto _label_5 :!via `PlayFromStart`)
            (else
              (goto _label_6))))))))

(event `StopMoving`
  ;[1 1 1] Move the Character
  (`|ExecutionSequence`
    (:`then_0`
      (goto _label_5 :!via `Stop`))
    (:`then_2`
      (`KismetSystemLibrary.Delay` 1.0)
      (`self.PickDirection`))))

(event `FindNextLocation`
  (bind _currentlocation (`self.CurrentLocation`))
  ;[1 1 1] Move the Character
  (switch `/Game/_LinkGame/Blueprints/Enums/E_FacingDirection` (`self.FacingDirection`)
    (:`NewEnumerator0`
      (set `self.NextLocation` (+ _currentlocation (* (100.0 0.0 0.0) 1))))
    (:`NewEnumerator1`
      (set `self.NextLocation` (+ _currentlocation (* (-100.0 0.0 0.0) 1))))
    (:`NewEnumerator2`
      (set `self.NextLocation` (+ _currentlocation (* (0.0 -100.0 0.0) 1))))
    (:`NewEnumerator3`
      (set `self.NextLocation` (+ _currentlocation (* (0.0 100.0 0.0) 1)))))
  (bind _inbounds (`self.CheckWithinAreaBounds`))
  (if (not _inbounds)
    (`KismetSystemLibrary.PrintString` "TOO FAR")
    (`self.StopMoving`)))

(event `ShootProjectile`
  (`KismetSystemLibrary.PrintString` "Shoot" true true (struct :`R` 1.0 :`A` 1.0) 10.0))

(event `self.ReceiveActorBeginOverlap`
  (params (OtherActor :type "Actor Object Reference"))
  ;[1 1 1] Collision
)

(event `self.StaticMesh.OnComponentHit`
  (params (HitComponent :type "PrimitiveComponent Object Reference") (OtherActor :type "Actor Object Reference") (OtherComp :type "PrimitiveComponent Object Reference") (NormalImpulse :type "Vector Structure") (Hit :type "HitResult Structure (by ref)"))
  ;[1 1 1] Collision
  (bind _astemp_player (cast `/Game/_LinkGame/Characters/Player/TempPlayer` OtherActor))
  (`GameplayStatics.ApplyDamage` _astemp_player (`self.AttackDamage`)))

(fn `CheckWithinAreaBounds`
  (returns (InBounds :type Boolean))
  (bind (_nextlocation_x _nextlocation_y) (`KismetMathLibrary.BreakVector` (`self.NextLocation`)))
  (bind (_zonecoords_x _zonecoords_y) (`KismetMathLibrary.BreakVector2D` (`self.ZoneCoords`)))
  (return (not (or (> (`KismetMathLibrary.Abs` (- (`KismetMathLibrary.Abs` _zonecoords_x) (`KismetMathLibrary.Abs` _nextlocation_x))) 500.0) (> (`KismetMathLibrary.Abs` (- (`KismetMathLibrary.Abs` _zonecoords_y) (`KismetMathLibrary.Abs` _nextlocation_y))) 700.0)))))

(fn `UserConstructionScript`)