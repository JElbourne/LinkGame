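; BP_Leever_Blue is the Blue Leever enemy Blueprint, which picks a new spot in its zone to move to.
; PickSpawnLocation resets TotalDistance, then repeatedly tries random points in a box around ZoneCoords until an object line trace hits nothing.
; The trace end re-rolls its random offsets, so it does not probe just beside the candidate point.
; On success it exits the loop, teleports the actor there and calls BurrowMovement.
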(fn `PickSpawnLocation`
  (bind (_zonecoords_x _zonecoords_y) (`KismetMathLibrary.BreakVector2D` (`self.ZoneCoords`)))
  (bind _returnvalue (`KismetMathLibrary.MakeVector` (+ _zonecoords_x (`KismetMathLibrary.RandomFloatInRange` -400.0 400.0)) (+ _zonecoords_y (`KismetMathLibrary.RandomFloatInRange` -600.0 600.0)) 20.0))
  (set `self.TotalDistance` 0)
  (for _ (range 51)
    (bind _output_get (set `self.WorldSpawnLocation` _returnvalue))
    (bind (_outhit _returnvalue_2) (`KismetSystemLibrary.LineTraceSingleForObjects` _output_get (+ _returnvalue (100.0 0.0 20.0)) (`self.Object Types`)))
    (if (not _returnvalue_2)
      (`|ExecutionSequence`
        (:`then_0`
          (break))
        (:`then_1`
          (`self.K2_SetActorLocationAndRotation` (`self.WorldSpawnLocation`) (`self.CurrentRotation`))
          (`self.BurrowMovement` false))))))

(fn `UserConstructionScript`
  (`parent.UserConstructionScript`))