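; BP_MenuController is the menu controller that creates the WB_MenuUI widget on BeginPlay and routes player input into it.
; The Select and Start inputs switch on the screen switcher's active index to drive the select, register or elimination mode widgets, with Start also entering mode selection from the first screen.
; WASD keys move the register screen's on-screen keyboard cursor directly, without checking which screen is active.
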(event `self.ReceiveBeginPlay`
  (bind _returnvalue (`|CreateWidget` "/Game/_LinkGame/UI/WB_MenuUI.WB_MenuUI_C" self))
  (bind _output_get (set `self.Menu UI` _returnvalue))
  (`UserWidget.AddToViewport` _output_get 0))

(event `InputAction|SelectButton`
  (params (Key :type "Key Structure"))
  (bind _menu_ui (`self.Menu UI`))
  (bind _menuscreenswitcher (`/Game/_LinkGame/UI/WB_MenuUI.MenuScreenSwitcher` (`self.Menu UI`)))
  (:`Pressed`
    (`/Engine/EditorBlueprintResources/StandardMacros.IsValid` _menuscreenswitcher
      (:`Is Valid`
        (switch `int` (`WidgetSwitcher.GetActiveWidgetIndex` _menuscreenswitcher)
          (:`1`
            (`/Game/_LinkGame/UI/WB_SelectMode.ChangeSelected` (`/Game/_LinkGame/UI/WB_MenuUI.WB_SelectMode` _menu_ui)))
          (:`2`
            (`/Game/_LinkGame/UI/WB_RegisterMode.ChangeSelected` (`/Game/_LinkGame/UI/WB_MenuUI.WB_RegisterMode` _menu_ui)))
          (:`3`
            (`/Game/_LinkGame/UI/WB_EliminationMode.ChangeSelected` (`/Game/_LinkGame/UI/WB_MenuUI.WB_EliminationMode` _menu_ui))))))))

(event `InputAction|StartButton`
  (params (Key :type "Key Structure"))
  (bind _menu_ui (`self.Menu UI`))
  (bind _wb_selectmode (`/Game/_LinkGame/UI/WB_MenuUI.WB_SelectMode` _menu_ui))
  (bind _menuscreenswitcher (`/Game/_LinkGame/UI/WB_MenuUI.MenuScreenSwitcher` (`self.Menu UI`)))
  (:`Pressed`
    (`/Engine/EditorBlueprintResources/StandardMacros.IsValid` _menuscreenswitcher
      (:`Is Valid`
        (switch `int` (`WidgetSwitcher.GetActiveWidgetIndex` _menuscreenswitcher)
          (:`0`
            (`/Game/_LinkGame/UI/WB_SelectMode.SwitchedToSelectMode` _wb_selectmode (`self.Menu UI`)))
          (:`1`
            (`/Game/_LinkGame/UI/WB_SelectMode.ChooseSelection` _wb_selectmode))
          (:`2`
            (`/Game/_LinkGame/UI/WB_RegisterMode.ChooseSelection` (`/Game/_LinkGame/UI/WB_MenuUI.WB_RegisterMode` _menu_ui)))
          (:`3`
            (`/Game/_LinkGame/UI/WB_EliminationMode.ChooseSelection` (`/Game/_LinkGame/UI/WB_MenuUI.WB_EliminationMode` _menu_ui))))))))

(event `Key|D`
  (params (Key :type "Key Structure"))
  (:`Pressed`
    (`/Game/_LinkGame/UI/WB_Keyboard.MoveCursorRight` (`/Game/_LinkGame/UI/WB_RegisterMode.WB_Keyboard` (`/Game/_LinkGame/UI/WB_MenuUI.WB_RegisterMode` (`self.Menu UI`))))))

(event `Key|A`
  (params (Key :type "Key Structure"))
  (:`Pressed`
    (`/Game/_LinkGame/UI/WB_Keyboard.MoveCurserLeft` (`/Game/_LinkGame/UI/WB_RegisterMode.WB_Keyboard` (`/Game/_LinkGame/UI/WB_MenuUI.WB_RegisterMode` (`self.Menu UI`))))))

(event `Key|W`
  (params (Key :type "Key Structure"))
  (:`Pressed`
    (`/Game/_LinkGame/UI/WB_Keyboard.MoveCursorUp` (`/Game/_LinkGame/UI/WB_RegisterMode.WB_Keyboard` (`/Game/_LinkGame/UI/WB_MenuUI.WB_RegisterMode` (`self.Menu UI`))))))

(event `Key|S`
  (params (Key :type "Key Structure"))
  (:`Pressed`
    (`/Game/_LinkGame/UI/WB_Keyboard.MoveCursorDown` (`/Game/_LinkGame/UI/WB_RegisterMode.WB_Keyboard` (`/Game/_LinkGame/UI/WB_MenuUI.WB_RegisterMode` (`self.Menu UI`))))))

(fn `UserConstructionScript`)