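; Octorok enemy for a Zelda-style game that wanders its zone on a 100-unit grid, sometimes shooting rocks, and damages the player on contact.
; Movement loops through a random new facing, optional shot and timeline-lerped steps, pausing when finished, out of bounds or overlapping non-players, with grid snapping on overlap.
; Death notifies the game state and drops items keyed by kill counter.
; It despawns when the camera finishes moving.
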(event `self.ReceiveBeginPlay`
  (`self.PickDirection`)
  (add `LinkMainCamera.OnFinishedMoving` (`self.CameraReference`) (delegate `DestroyEnemy`))
  (set `self.Health` 1.0))

(event `DestroyEnemy`
  (`self.K2_DestroyActor`))

(event `self.Die`
  ;[1 1 1] On Death
  (bind _asbp_link_game_state (cast `/Game/_LinkGame/Blueprints/BP_LinkGameState` (`GameplayStatics.GetGameState`)))
  (bind _output_get (set `self.As BP Link Game State` _asbp_link_game_state))
  (`/Game/_LinkGame/Blueprints/BP_LinkGameState.EnemyDied` _output_get (`self.EnemyId`))
  (`self.DropItem`)
  (`self.K2_DestroyActor`))

(event `DropItem`
  ;[1 1 1] On Death
  (bind _killcounter (`/Game/_LinkGame/Blueprints/BP_LinkGameState.IncrementKillCounter` (`self.As BP Link Game State`)))
  (switch `int` (`KismetMathLibrary.RandomInteger` 3)
    (:`0`
      _)
    (:`1`
      _)
    (:`2`
      _))
  (bind (_value _returnvalue) (`BlueprintMapLibrary.Map_Find` (`self.ItemDropChoices`) _killcounter))
  (if _returnvalue
    (`|SpawnActorFromClass` _value (`KismetMathLibrary.MakeTransform` (`self.K2_GetActorLocation`)) "Undefined" "OverrideRootScale" null null false null)))

(event `PickDirection`
  (bind _facingdirection (`self.FacingDirection`))
  ;[1 1 1] Move the Character
  ;;[1 1 1] Pick Rotation
  (switch `int` (`KismetMathLibrary.RandomInteger` 4)
    (:`0`
      (if (`|EnumEquality` _facingdirection "NewEnumerator0")
        (`self.PickDirection` :!label _label)
        (else
          (set `self.CurrentRotation` (struct))
          (set `self.FacingDirection` "NewEnumerator0")
          (`self.K2_SetActorRotation` (`self.CurrentRotation`) :!label _label_2)
          (switch `int` (`KismetMathLibrary.RandomInteger` 5)
            (:`0`
              (`self.MoveForward` :!label _label_3))
            (:`1`
              (goto _label_3))
            (:`2`
              (goto _label_3))
            (:`3`
              (`self.ShootProjectile` :!label _label_4)
              (`self.MoveForward`))
            (:`4`
              (goto _label_4))))))
    (:`1`
      (if (`|EnumEquality` _facingdirection "NewEnumerator2")
        (goto _label)
        (else
          (set `self.CurrentRotation` (struct :`Yaw` 270.0))
          (set `self.FacingDirection` "NewEnumerator2")
          (goto _label_2))))
    (:`2`
      (if (`|EnumEquality` _facingdirection "NewEnumerator1")
        (goto _label)
        (else
          (set `self.CurrentRotation` (struct :`Yaw` 180.0))
          (set `self.FacingDirection` "NewEnumerator1")
          (goto _label_2))))
    (:`3`
      (if (`|EnumEquality` _facingdirection "NewEnumerator3")
        (goto _label)
        (else
          (set `self.CurrentRotation` (struct :`Yaw` 90.0))
          (set `self.FacingDirection` "NewEnumerator3")
          (goto _label_2))))))

(event `MoveForward`
  (bind (_returnvalue_x _returnvalue_y _returnvalue_z) (`KismetMathLibrary.BreakVector` (`self.K2_GetActorLocation`)))
  ;[1 1 1] Move the Character
  (set `self.CurrentLocation` (`self.K2_GetActorLocation`))
  (`self.FindNextLocation`)
  (set `self.RandomDistance` (+ (`KismetMathLibrary.RandomInteger` 5) 1))
  (`self.Timeline_EnemyWalk` :!label _label_5
    (:`then`
      (bind (_direction _amountmoved) (`Timeline|Timeline_EnemyWalk` :!via `PlayFromStart` :!label _label_6)
        (:`Update`
          (bind _inbounds (`self.CheckWithinAreaBounds`))
          (if _inbounds
            (bind (_sweephitresult _returnvalue) (`self.K2_SetActorLocation` (`KismetMathLibrary.VLerp` (`self.CurrentLocation`) (`self.NextLocation`) _amountmoved)))
            (if (not _returnvalue)
              (`self.StopMoving`)
              (`self.K2_SetActorLocation` (`KismetMathLibrary.MakeVector` (* (`KismetMathLibrary.Round` (/ _returnvalue_x 100.0)) 100.0) (+ (* (`KismetMathLibrary.Round` (/ (- _returnvalue_y 50.0) 100.0)) 100.0) 50.0) _returnvalue_z)))
            (else
              (`self.StopMoving` :!label _label_7))))
        (:`Finished`
          (bind _result (`/Engine/EditorBlueprintResources/StandardMacros.DecrementInt` (`self.RandomDistance`))
            (:`  `
              (if (> _result 0)
                (set `self.CurrentLocation` (`self.NextLocation`))
                (`self.FindNextLocation`)
                (goto _label_5)
                (else
                  (goto _label_7))))))))
    (:`else`)))

(event `StopMoving`
  ;[1 1 1] Move the Character
  (`|ExecutionSequence`
    (:`then_0`
      (goto _label_6 :!via `Stop`))
    (:`then_1`
      (`KismetSystemLibrary.Delay` 1.0)
      (`self.PickDirection`))))

(event `FindNextLocation`
  (bind _currentlocation (`self.CurrentLocation`))
  ;[1 1 1] Move the Character
  (switch `/Game/_LinkGame/Blueprints/Enums/E_FacingDirection` (`self.FacingDirection`)
    (:`NewEnumerator0`
      (set `self.NextLocation` (+ _currentlocation (* (100.0 0.0 0.0) 1))))
    (:`NewEnumerator1`
      (set `self.NextLocation` (+ _currentlocation (* (-100.0 0.0 0.0) 1))))
    (:`NewEnumerator2`
      (set `self.NextLocation` (+ _currentlocation (* (0.0 -100.0 0.0) 1))))
    (:`NewEnumerator3`
      (set `self.NextLocation` (+ _currentlocation (* (0.0 100.0 0.0) 1)))))
  (bind _inbounds (`self.CheckWithinAreaBounds`))
  (if (not _inbounds)
    (`self.StopMoving`)))

(event `ShootProjectile`
  (bind (_returnvalue_location _returnvalue_rotation) (`KismetMathLibrary.BreakTransform` (`self.GetTransform`)))
  (bind _arrow (`self.Arrow`))
  (`/Engine/EditorBlueprintResources/StandardMacros.IsValid` _arrow
    (:`Is Valid`
      (`|SpawnActorFromClass` "/Game/_LinkGame/Blueprints/Projectile/BP_RockProjectile.BP_RockProjectile_C" (`KismetMathLibrary.MakeTransform` (`SceneComponent.K2_GetComponentLocation` _arrow) _returnvalue_rotation (0.4 0.4 0.4)) "AlwaysSpawn" "OverrideRootScale" self (0.0 0.0) 0.5 null))))

(event `self.StaticMesh.OnComponentBeginOverlap`
  (params (OverlappedComponent :type "PrimitiveComponent Object Reference") (OtherActor :type "Actor Object Reference") (OtherComp :type "PrimitiveComponent Object Reference") (OtherBodyIndex :type Integer) (bFromSweep :type Boolean) (SweepResult :type "HitResult Structure (by ref)"))
  (bind (_returnvalue_x _returnvalue_y _returnvalue_z) (`KismetMathLibrary.BreakVector` (`self.K2_GetActorLocation`)))
  ;[1 1 1] Collision
  (bind _astemp_player (cast `/Game/_LinkGame/Characters/Player/TempPlayer` OtherActor)
    (:`then`
      (if (== OtherComp (`Character.CapsuleComponent` _astemp_player))
        (`GameplayStatics.ApplyDamage` _astemp_player (`self.AttackDamage`))))
    (:`CastFailed`
      (`self.StopMoving`)
      (`KismetSystemLibrary.PrintString` "Hello")
      (`self.K2_SetActorLocation` (`KismetMathLibrary.MakeVector` (* (`KismetMathLibrary.Round` (/ _returnvalue_x 100.0)) 100.0) (+ (* (`KismetMathLibrary.Round` (/ (- _returnvalue_y 50.0) 100.0)) 100.0) 50.0) _returnvalue_z)))))

(fn `CheckWithinAreaBounds`
  (returns (InBounds :type Boolean))
  (bind (_zonecoords_x _zonecoords_y) (`KismetMathLibrary.BreakVector2D` (`self.ZoneCoords`)))
  (bind (_nextlocation_x _nextlocation_y) (`KismetMathLibrary.BreakVector` (`self.NextLocation`)))
  (return (not (or (> (`KismetMathLibrary.Abs` (- (`KismetMathLibrary.Abs` _zonecoords_x) (`KismetMathLibrary.Abs` _nextlocation_x))) 500.0) (> (`KismetMathLibrary.Abs` (- (`KismetMathLibrary.Abs` _zonecoords_y) (`KismetMathLibrary.Abs` _nextlocation_y))) 700.0)))))

(fn `UserConstructionScript`)