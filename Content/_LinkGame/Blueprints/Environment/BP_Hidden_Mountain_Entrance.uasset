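; BP_Hidden_Mountain_Entrance is an overworld cave entrance hidden behind a mountain component that a bomb can open.
; Bomb damage runs once, revealing the door, destroying the mountain, playing the secret sound and saving the cave as unhidden in the game instance's cave map by CaveID.
; UpdateCaveData extends the parent's version, showing the door and removing the mountain when the cave data is not hidden.
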(event `self.UpdateCaveData`
  (bind (_cavedata_npc _cavedata_dialogueline1 _cavedata_dialogueline2 _cavedata_bisitemsconditionmet _cavedata_bisonetimeuse _cavedata_biscavecompleted _cavedata_bisdirty _cavedata_item1 _cavedata_item2 _cavedata_item3 _cavedata_hidden) (break `/Game/_LinkGame/Structs/ST_CaveData` (`self.CaveData`)))
  (bind _mountain (`self.Mountain`))
  (`parent.UpdateCaveData`)
  (if (not _cavedata_hidden)
    (`SceneComponent.SetVisibility` (`self.Door`) true false)
    (`/Engine/EditorBlueprintResources/StandardMacros.IsValid` _mountain
      (:`Is Valid`
        (`ActorComponent.K2_DestroyComponent` _mountain)))))

(event `/Game/_LinkGame/Blueprints/Interface/I_Damage.TakeDamageFromBomb`
  (params (Damage :type "Float (single-precision)"))
  (bind _mountain (`self.Mountain`))
  (bind _caveid (`self.CaveID`))
  (bind _overworldcavedata (`/Game/_LinkGame/Blueprints/BP_Link_GameInstance.OverworldCaveData` (`self.As BP Link Game Instance`)))
  (bind (_value _returnvalue) (`BlueprintMapLibrary.Map_Find` (`/Game/_LinkGame/Blueprints/BP_Link_GameInstance.OverworldCaveData` (`self.As BP Link Game Instance`)) (`self.CaveID`)))
  (`/Engine/EditorBlueprintResources/StandardMacros.DoOnce` false
    (:`Completed`
      (`SceneComponent.SetVisibility` (`self.Door`) true false)
      (`/Engine/EditorBlueprintResources/StandardMacros.IsValid` _mountain
        (:`Is Valid`
          (`ActorComponent.K2_DestroyComponent` _mountain)
          (`GameplayStatics.PlaySound2D` "/Game/_LinkGame/Audio/SoundEffects/LOZ_Secret.LOZ_Secret" 1.0 1.0 0.0 null null)
          (if _returnvalue
            (bind _structout (setmembers `/Game/_LinkGame/Structs/ST_CaveData` :`StructRef` _value :`Hidden` false))
            (`BlueprintMapLibrary.Map_Add` _overworldcavedata _caveid _structout)
            (else
              (bind _structout_2 (setmembers `/Game/_LinkGame/Structs/ST_CaveData` :`StructRef` (`self.CaveData`) :`Hidden` false))
              (`BlueprintMapLibrary.Map_Add` _overworldcavedata _caveid _structout_2))))))))

(fn `UserConstructionScript`
  (`parent.UserConstructionScript`))