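; Bomb weapon actor that starts its countdown on spawn, explodes to damage nearby actors, then destroys itself.
; One timeline expands the overlap sphere toward DamageRadius; its Countdown event enables overlaps and plays the blast sound.
; Overlapped components whose object type is in EffectingActors trigger a bomb-damage message to their actor.
; When the mesh overlaps a custom channel, apparently mountains, the bomb moves to a fixed height and prints debug text.
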(event `self.ReceiveBeginPlay`
  (bind _sphere (`self.Sphere`))
  (`SphereComponent.SetSphereRadius` _sphere 30.0 false)
  (set `PrimitiveComponent.bGenerateOverlapEvents` false _sphere)
  (bind (_direction _growth) (`Timeline|Timeline_Explode` :!via `PlayFromStart`)
    (:`Update`
      (`SphereComponent.SetSphereRadius` (`self.Sphere`) (`KismetMathLibrary.Lerp` 30.0 (`self.DamageRadius`) _growth) true))
    (:`Finished`
      (`self.K2_DestroyActor`))
    (:`Countdown`
      (set `PrimitiveComponent.bGenerateOverlapEvents` true (`self.Sphere`))
      (`GameplayStatics.PlaySound2D` "/Game/_LinkGame/Audio/SoundEffects/LOZ_Bomb_Blow.LOZ_Bomb_Blow" 1.0 1.0 0.0 null null))))

(event `self.Sphere.OnComponentBeginOverlap`
  (params (OverlappedComponent :type "PrimitiveComponent Object Reference") (OtherActor :type "Actor Object Reference") (OtherComp :type "PrimitiveComponent Object Reference") (OtherBodyIndex :type Integer) (bFromSweep :type Boolean) (SweepResult :type "HitResult Structure (by ref)"))
  (if (`KismetArrayLibrary.Array_Contains` (`self.EffectingActors`) (`PrimitiveComponent.GetCollisionObjectType` OtherComp))
    (message `/Game/_LinkGame/Blueprints/Interface/I_Damage.TakeDamageFromBomb` OtherActor (`self.Damage`))))

(event `self.StaticMesh.OnComponentBeginOverlap`
  (params (OverlappedComponent :type "PrimitiveComponent Object Reference") (OtherActor :type "Actor Object Reference") (OtherComp :type "PrimitiveComponent Object Reference") (OtherBodyIndex :type Integer) (bFromSweep :type Boolean) (SweepResult :type "HitResult Structure (by ref)"))
  (bind (_returnvalue_x _returnvalue_y) (`KismetMathLibrary.BreakVector` (`self.K2_GetActorLocation`)))
  (if (`|EnumEquality` (`PrimitiveComponent.GetCollisionObjectType` OtherComp) "ECC_GameTraceChannel7")
    (`KismetSystemLibrary.PrintString` "Moutain")
    (`self.K2_SetActorLocation` (`KismetMathLibrary.MakeVector` _returnvalue_x _returnvalue_y 100.0))))

(fn `UserConstructionScript`)