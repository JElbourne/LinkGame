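; BP_Boulder is an enemy hazard that repeatedly hops along -X with random sideways drift, damaging the player on capsule overlap.
; A timeline lerps each hop toward a random next point with an arced height; overlapping a non-player while falling ends it and records the landing height.
; After each hop, leaving the bounds around ZoneCoords respawns it at the zone's +X edge.
; It destroys itself when the referenced camera finishes moving.
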(event `self.ReceiveBeginPlay`
  (add `LinkMainCamera.OnFinishedMoving` (`self.CameraReference`) (delegate `DestroyEnemy`))
  (`self.PickSpawnLocation`)
  (`self.PickNextLocation`))

(event `DestroyEnemy`
  (`self.K2_DestroyActor`))

(event `PickNextLocation`
  (bind (_returnvalue_x _returnvalue_y) (`KismetMathLibrary.BreakVector` (`self.K2_GetActorLocation`)))
  (set `self.NextLocation` (`KismetMathLibrary.MakeVector` (+ _returnvalue_x (`KismetMathLibrary.RandomFloatInRange` -200.0 -300.0)) (+ _returnvalue_y (`KismetMathLibrary.RandomFloatInRange` -300.0 300.0))))
  (`self.JumpToLocation`))

(event `JumpToLocation`
  (bind _output_get (set `self.CurrentLocation` (`self.K2_GetActorLocation`)))
  (if (> (`KismetMathLibrary.Vector_Distance` _output_get (`self.NextLocation`)) 250.0)
    (`self.Timeline_JumpTo`
      (:`then`
        (bind (_direction _travelpercentage _jumpheightpercentage) (`Timeline|Timeline_JumpTo` :!via `PlayFromStart` :!label _label)
          (:`Update`
            (bind (_returnvalue_x _returnvalue_y) (`KismetMathLibrary.BreakVector` (`KismetMathLibrary.VLerp` (`self.CurrentLocation`) (`self.NextLocation`) _travelpercentage)))
            (`self.K2_SetActorLocation` (`KismetMathLibrary.MakeVector` _returnvalue_x _returnvalue_y (`KismetMathLibrary.Lerp` (`self.LastHeight`) (`self.JumpHeight`) _jumpheightpercentage))))
          (:`Finished`
            (`self.StopMoving`))
          (:`Falling`
            (set `self.Falling` true)
            (set `self.LastHeight` 0.0))))
      (:`else`))
    (else
      (`self.StopMoving`))))

(event `StopMoving`
  (`|ExecutionSequence`
    (:`then_0`
      (goto _label :!via `Stop`))
    (:`then_1`
      (`KismetSystemLibrary.Delay` 0.1)
      (`self.CheckIfInBounds`)
      (`self.PickNextLocation`)
      (set `self.Falling` false))))

(event `self.StaticMesh.OnComponentBeginOverlap`
  (params (OverlappedComponent :type "PrimitiveComponent Object Reference") (OtherActor :type "Actor Object Reference") (OtherComp :type "PrimitiveComponent Object Reference") (OtherBodyIndex :type Integer) (bFromSweep :type Boolean) (SweepResult :type "HitResult Structure (by ref)"))
  (bind (_returnvalue_x _returnvalue_y _returnvalue_z) (`KismetMathLibrary.BreakVector` (`self.K2_GetActorLocation`)))
  ;[1 1 1] Collision
  (bind _astemp_player (cast `/Game/_LinkGame/Characters/Player/TempPlayer` OtherActor)
    (:`then`
      (if (== OtherComp (`Character.CapsuleComponent` _astemp_player))
        (`GameplayStatics.ApplyDamage` _astemp_player (`self.Damage`))))
    (:`CastFailed`
      (if (`self.Falling`)
        (`self.StopMoving`)
        (set `self.LastHeight` _returnvalue_z)))))

(event `CheckIfInBounds`
  (bind (_returnvalue_x _returnvalue_y) (`KismetMathLibrary.BreakVector` (`self.K2_GetActorLocation`)))
  (bind (_zonecoords_x _zonecoords_y) (`KismetMathLibrary.BreakVector2D` (`self.ZoneCoords`)))
  (if (or (> (`KismetMathLibrary.Abs` (- (`KismetMathLibrary.Abs` _zonecoords_x) (`KismetMathLibrary.Abs` _returnvalue_x))) 500.0) (> (`KismetMathLibrary.Abs` (- (`KismetMathLibrary.Abs` _zonecoords_y) (`KismetMathLibrary.Abs` _returnvalue_y))) 700.0))
    (`self.PickSpawnLocation`)))

(event `PickSpawnLocation`
  (bind (_zonecoords_x _zonecoords_y) (`KismetMathLibrary.BreakVector2D` (`self.ZoneCoords`)))
  (bind _output_get (set `self.LastHeight` 110.0))
  (`self.K2_SetActorLocation` (`KismetMathLibrary.MakeVector` (+ _zonecoords_x 500.0) (`KismetMathLibrary.RandomFloatInRange` (- _zonecoords_y 500.0) (+ _zonecoords_y 500.0)) _output_get)))

(fn `UserConstructionScript`)