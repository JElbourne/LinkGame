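; BP_HeartContainer is a heart container pickup that raises the player's health capacity.
; When its mesh overlaps TempPlayer, it calls HealthContainerPickup with one unit and destroys itself, while sword projectiles are ignored.
; Pickups flagged as special overworld items first report their location to the Link game instance, cached at BeginPlay, through PickedUpOverworldItem.
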(event `self.ReceiveBeginPlay`
  (`parent.ReceiveBeginPlay`)
  (bind _asbp_link_game_instance (cast `/Game/_LinkGame/Blueprints/BP_Link_GameInstance` (`GameplayStatics.GetGameInstance`)))
  (set `self.As BP Link Game Instance` _asbp_link_game_instance))

(event `self.ItemStaticMesh.OnComponentBeginOverlap`
  (params (OverlappedComponent :type "PrimitiveComponent Object Reference") (OtherActor :type "Actor Object Reference") (OtherComp :type "PrimitiveComponent Object Reference") (OtherBodyIndex :type Integer) (bFromSweep :type Boolean) (SweepResult :type "HitResult Structure (by ref)"))
  (cast `/Game/_LinkGame/Blueprints/Weapons/Projectile/BP_SwordProjectile` OtherActor
    (:`CastFailed`
      (bind _astemp_player (cast `/Game/_LinkGame/Characters/Player/TempPlayer` OtherActor))
      (`/Game/_LinkGame/Characters/Player/TempPlayer.HealthContainerPickup` _astemp_player 1.0)
      (if (`self.IsSpecialOverworldItem`)
        (`/Game/_LinkGame/Blueprints/BP_Link_GameInstance.PickedUpOverworldItem` (`self.As BP Link Game Instance`) (`self.K2_GetActorLocation`)))
      (`self.K2_DestroyActor`))))

(fn `UserConstructionScript`
  (`parent.UserConstructionScript`))