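; White Sword pickup Blueprint that gives the player a sword once their max health meets a heart requirement.
; It overrides PickupandDestroy, comparing the player's MaxHealth to HeartsRequired before passing its mesh and damage to PickUpSword.
; After a successful pickup it notifies its spawner through ItemPickedUp, or destroys itself when no valid spawner exists.
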(event `self.PickupAndDestroy`
  (bind (_playerdata_health _playerdata_maxhealth) (break `/Game/_LinkGame/Structs/ST_PlayerData` (`/Game/_LinkGame/Characters/Player/TempPlayer.PlayerData` (`self.As Temp Player`))))
  (if (>= _playerdata_maxhealth (`KismetMathLibrary.Conv_IntToDouble` (`self.HeartsRequired`)))
    (`/Game/_LinkGame/Characters/Player/TempPlayer.PickUpSword` (`self.As Temp Player`) (`StaticMeshComponent.StaticMesh` (`self.ItemStaticMesh`)) (`self.Damage`))
    (bind _spawnerreference (`self.SpawnerReference`)
      (:`then`
        (`/Game/_LinkGame/Blueprints/Actors/BP_CaveSpawner.ItemPickedUp` _spawnerreference (`self.As Temp Player`) self))
      (:`else`
        (`self.K2_DestroyActor`)))))

(fn `UserConstructionScript`
  (`parent.UserConstructionScript`))