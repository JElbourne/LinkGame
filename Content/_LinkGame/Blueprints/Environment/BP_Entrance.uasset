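; Level transition actor that moves the player between the overworld and caves by opening a named level.
; On overlap it freezes and centers the player, then hands PlayerData, travel direction and, unless the stored cave is completed, its CaveData to the game instance.
; Before entering a cave it saves camera and Arrow locations for the overworld.
; On BeginPlay after returning to the overworld, it takes back the stored CaveData and resets it.
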(event `self.ReceiveBeginPlay`
  (bind _asbp_link_game_instance (cast `/Game/_LinkGame/Blueprints/BP_Link_GameInstance` (`GameplayStatics.GetGameInstance`)))
  (set `self.As BP Link Game Instance` _asbp_link_game_instance)
  (bind _asbp_player_controller (cast `/Game/_LinkGame/Blueprints/Controllers/BP_PlayerController` (`GameplayStatics.GetPlayerController` 0)))
  (set `self.As BP Player Controller` _asbp_player_controller)
  (`self.UpdateCaveData`))

(event `UpdateCaveData`
  (bind _as_bp_link_game_instance (`self.As BP Link Game Instance`))
  (if (`/Game/_LinkGame/Blueprints/BP_Link_GameInstance.IsTravelingToOverworld` _as_bp_link_game_instance)
    (set `self.CaveData` (`/Game/_LinkGame/Blueprints/BP_Link_GameInstance.CaveData` _as_bp_link_game_instance))
    (set `/Game/_LinkGame/Blueprints/BP_Link_GameInstance.CaveData` (make `/Game/_LinkGame/Structs/ST_CaveType` "/Game/_LinkGame/Characters/NPC/BP_NPCBase.BP_NPCBase_C" "" "" false false false false "/Game/_LinkGame/Blueprints/Pickups/BP_Base_Pickup.BP_Base_Pickup_C" "/Game/_LinkGame/Blueprints/Pickups/BP_Base_Pickup.BP_Base_Pickup_C" "/Game/_LinkGame/Blueprints/Pickups/BP_Base_Pickup.BP_Base_Pickup_C") (`self.As BP Link Game Instance`))))

(event `self.Collider.OnComponentBeginOverlap`
  (params (OverlappedComponent :type "PrimitiveComponent Object Reference") (OtherActor :type "Actor Object Reference") (OtherComp :type "PrimitiveComponent Object Reference") (OtherBodyIndex :type Integer) (bFromSweep :type Boolean) (SweepResult :type "HitResult Structure (by ref)"))
  (bind (_returnvalue_x _returnvalue_y) (`KismetMathLibrary.BreakVector` (`self.K2_GetActorLocation`)))
  (bind _as_bp_link_game_instance (`self.As BP Link Game Instance`))
  (bind _as_bp_link_game_instance_2 (`self.As BP Link Game Instance`))
  (bind (_cavedata_npc _cavedata_dialogueline1 _cavedata_dialogueline2 _cavedata_bisitemsconditionmet _cavedata_bisonetimeuse _cavedata_biscavecompleted) (break `/Game/_LinkGame/Structs/ST_CaveType` (`/Game/_LinkGame/Blueprints/BP_Link_GameInstance.CaveData` _as_bp_link_game_instance)))
  (bind _astemp_player (cast `/Game/_LinkGame/Characters/Player/TempPlayer` OtherActor))
  (set `LinkGameCharacter.bIsMovementFrozen` true _astemp_player)
  (set `/Game/_LinkGame/Blueprints/BP_Link_GameInstance.PlayerData` (`/Game/_LinkGame/Characters/Player/TempPlayer.PlayerData` _astemp_player) _as_bp_link_game_instance)
  (if (not _cavedata_biscavecompleted)
    (set `/Game/_LinkGame/Blueprints/BP_Link_GameInstance.CaveData` (`self.CaveData`) _as_bp_link_game_instance))
  (bind (_returnvalue_x_2 _returnvalue_y_2 _returnvalue_z) (`KismetMathLibrary.BreakVector` (`self.K2_GetActorLocation` _astemp_player)))
  (`self.K2_SetActorLocation` _astemp_player (`KismetMathLibrary.MakeVector` _returnvalue_x _returnvalue_y _returnvalue_z) false false)
  (bind _output_get (set `/Game/_LinkGame/Blueprints/BP_Link_GameInstance.IsTravelingToOverworld` (`self.bIsTravelToOverworld`) (`self.As BP Link Game Instance`)))
  (if _output_get
    (`KismetSystemLibrary.Delay` 0.25)
    (else
      ;[1 1 1] For future Animation
      (`KismetSystemLibrary.Delay` 1.0)
      (set `/Game/_LinkGame/Blueprints/BP_Link_GameInstance.OverworldCameraLocation` (`SceneComponent.K2_GetComponentLocation` (`/Game/_LinkGame/Blueprints/Cameras/BP_MainCamera.DefaultSceneRoot` (`/Game/_LinkGame/Blueprints/Controllers/BP_PlayerController.CurrentCamera` (`self.As BP Player Controller`)))) _as_bp_link_game_instance_2)
      (set `/Game/_LinkGame/Blueprints/BP_Link_GameInstance.OverworldPlayerLocation` (`SceneComponent.K2_GetComponentLocation` (`self.Arrow`)) _as_bp_link_game_instance_2)))
  (`GameplayStatics.OpenLevel` (`self.Level Name`)))

(fn `UserConstructionScript`)