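; Player controller for the Link game that handles camera registration, pausing and a jump to the game over level.
; It caches the TempPlayer character on BeginPlay and switches the view target to whichever main camera registers with it.
; SelectButton toggles pause through a FlipFlop.
; Escape copies the player's PlayerData into BP_Link_GameInstance, then opens L_GameOver.
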(event `self.ReceiveBeginPlay`
  (bind _astemp_player (cast `/Game/_LinkGame/Characters/Player/TempPlayer` (`GameplayStatics.GetPlayerCharacter` 0)))
  (set `self.As Temp Player` _astemp_player))

(event `RegisterMainCamera`
  (params (MainCamera :type "/Game/_LinkGame/Blueprints/Cameras/BP_MainCamera Object Reference"))
  (bind _output_get (set `self.CurrentCamera` MainCamera))
  (`self.SetViewTargetWithBlend` self _output_get 0.0 "VTBlend_Linear" 0.0 false))

(event `InputAction|SelectButton` :paused true
  (params (Key :type "Key Structure"))
  (:`Pressed`
    (bind _isa (`/Engine/EditorBlueprintResources/StandardMacros.FlipFlop`)
      (:`A`
        _)
      (:`B`
        _))
    (`GameplayStatics.SetGamePaused` _isa)))

(event `Key|Escape`
  (params (Key :type "Key Structure"))
  (:`Pressed`
    (bind _asbp_link_game_instance (cast `/Game/_LinkGame/Blueprints/BP_Link_GameInstance` (`GameplayStatics.GetGameInstance`)))
    (set `/Game/_LinkGame/Blueprints/BP_Link_GameInstance.PlayerData` (`/Game/_LinkGame/Characters/Player/TempPlayer.PlayerData` (`self.As Temp Player`)) _asbp_link_game_instance)
    (`GameplayStatics.OpenLevel` "L_GameOver")))

(fn `UserConstructionScript`)